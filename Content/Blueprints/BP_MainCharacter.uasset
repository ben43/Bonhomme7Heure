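; BP_MainCharacter is the player character Blueprint, handling camera look, movement, grabbing and interaction input.
; Movement axes call MoveForward and MoveRight from C++, while GrabInput press and release drive the C++ Grabber component.
; Interact runs a debug-drawn Visibility line trace from the follow camera out to Reach, notifying any BP_MusicKey hit.
; A fallback cast to BP_HiddenActor triggers nothing further.
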(event EventBeginPlay
  ;[1 1 1] BeginPlay
)

(event Input|ActionEvents|InputActionInteract
  (params (Key :type Key%20Structure :default "None"))
  (bind _followcamera (Variables|Default|GetFollowCamera))
  (bind _returnvalue (Transformation|GetWorldLocation _followcamera))
  (:Pressed
    (bind (_outhit _returnvalue_2) (Collision|LineTraceByChannel _returnvalue (+ _returnvalue (* (Math|Vector|GetForwardVector _followcamera) (Variables|Default|GetReach))) "TraceTypeQuery1" false 0 "ForDuration"))
    (if _returnvalue_2
      (bind _asbp_music_key (Utilities|Casting|CastToBP_MusicKey (.HitActor (Collision|BreakHitResult _outhit)))
        (:then
          (Default|PlayerInteractionAttempt _asbp_music_key))
        (:CastFailed
          (Utilities|Casting|CastToBP_HiddenActor (.HitActor (Collision|BreakHitResult _outhit))))))))

(event Input|ActionEvents|InputActionGrabInput
  (params (Key :type Key%20Structure :default "None"))
  (bind _grabber1 (Variables|Default|GetGrabber1))
  ;[1 1 1] Call the Grabber from Grabber.cpp
  (:Pressed
    (Class|Grabber|Grab _grabber1))
  (:Released
    (Class|Grabber|Release _grabber1)))

(event Input|AxisEvents|InputAxisTurnCamera
  (params (AxisValue :type Float%20%28single-precision%29))
  ;[1 1 1] Call Movement from .cpp file
  (Pawn|Input|AddControllerYawInput AxisValue))

(event Input|AxisEvents|InputAxisMoveForward
  (params (AxisValue :type Float%20%28single-precision%29))
  ;[1 1 1] Call Movement from .cpp file
  (Class|MainCharacter|MoveForward AxisValue))

(event Input|AxisEvents|InputAxisMoveRight
  (params (AxisValue :type Float%20%28single-precision%29))
  ;[1 1 1] Call Movement from .cpp file
  (Class|MainCharacter|MoveRight AxisValue))

(event Input|AxisEvents|InputAxisLookUpCamera
  (params (AxisValue :type Float%20%28single-precision%29))
  ;[1 1 1] Call Movement from .cpp file
  (Pawn|Input|AddControllerPitchInput AxisValue))

(fn ConstructionScript)