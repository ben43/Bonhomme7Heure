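; BP_LoreItem is an interactable lore pickup whose mesh is set from a variable in the construction script.
; A Box overlap adds an interact prompt widget when BP_MainCharacter enters and removes it on exit.
; Interact plays a book pickup sound at the mesh and opens the diary widget, passing the item itself as LoreItem.
; The item is not destroyed or hidden afterward.
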(event OnComponentBeginOverlap(Box)
  (params (OverlappedComponent :type Primitive%20Component%20Object%20Reference) (OtherActor :type Actor%20Object%20Reference) (OtherComp :type Primitive%20Component%20Object%20Reference) (OtherBodyIndex :type Integer) (bFromSweep :type Boolean) (SweepResult :type Hit%20Result%20Structure%20%28by%20ref%29))
  (Utilities|Casting|CastToBP_MainCharacter OtherActor)
  (bind _returnvalue (UserInterface|CreateWidget "/Game/UI/BP_WGT_Interact.BP_WGT_Interact_C"))
  (UserInterface|Viewport|AddtoViewport _returnvalue 0))

(event OnComponentEndOverlap(Box)
  (params (OverlappedComponent :type Primitive%20Component%20Object%20Reference) (OtherActor :type Actor%20Object%20Reference) (OtherComp :type Primitive%20Component%20Object%20Reference) (OtherBodyIndex :type Integer))
  (Utilities|Casting|CastToBP_MainCharacter OtherActor)
  (Widget|RemovefromParent (stale OnComponentBeginOverlap(Box) _returnvalue)))

(event EventInteract
  (params (FromEnigma? :type Boolean))
  (Audio|SpawnSoundatLocation "/Game/Sounds/SFX/Diary/BookPicking01.BookPicking01" (Transformation|GetWorldLocation (Variables|Default|GetStaticMesh)) "0, 0, 0" 1.0 1.0 0.0 "/Game/Sounds/Attenuations/Footstep.Footstep" 0)
  (bind _returnvalue (UserInterface|CreateWidget "/Game/UI/BP_WGT_Diary_Main.BP_WGT_Diary_Main_C" (Game|GetPlayerController 0) self))
  (UserInterface|Viewport|AddtoViewport _returnvalue 0))

(fn ConstructionScript
  (Components|StaticMesh|SetStaticMesh (Variables|Default|GetStaticMesh) (Variables|Default|GetMesh)))