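; BP_MusicMaster is the master actor of a music puzzle (enigma) that plays a sound when the player interacts nearby.
; Box overlaps with BP_MainCharacter toggle CanInteract and create or remove an interact widget, which is never added to the viewport here.
; SoundSequenceVerification loops over key references, advancing or resetting a sequence counter, with completion only printed.
; Its element check compares against the array itself, and nothing here calls it.
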(event OnComponentBeginOverlap(Box)
  (params (OverlappedComponent :type Primitive%20Component%20Object%20Reference) (OtherActor :type Actor%20Object%20Reference) (OtherComp :type Primitive%20Component%20Object%20Reference) (OtherBodyIndex :type Integer) (bFromSweep :type Boolean) (SweepResult :type Hit%20Result%20Structure%20%28by%20ref%29))
  (Utilities|Casting|CastToBP_MainCharacter OtherActor)
  (bind _returnvalue (UserInterface|CreateWidget "/Game/UI/BP_WGT_Interact.BP_WGT_Interact_C" (Game|GetPlayerController 0)))
  (Variables|Default|SetInteractPrompt _returnvalue)
  (Variables|Default|SetCanInteract true))

(event OnComponentEndOverlap(Box)
  (params (OverlappedComponent :type Primitive%20Component%20Object%20Reference) (OtherActor :type Actor%20Object%20Reference) (OtherComp :type Primitive%20Component%20Object%20Reference) (OtherBodyIndex :type Integer))
  (Utilities|Casting|CastToBP_MainCharacter OtherActor)
  (Widget|RemovefromParent (Variables|Default|GetInteractPrompt))
  (Variables|Default|SetCanInteract false))

(event Custom|InteractAttempt
  (if (Variables|Default|GetCanInteract)
    (Audio|Components|Audio|Play (Variables|Default|GetMusicToPlay) 0.0)))

(event EventBeginPlay)

(event Collision|EventActorBeginOverlap
  (params (OtherActor :type Actor%20Object%20Reference)))

(event EventTick
  (params (DeltaSeconds :type Float%20%28single-precision%29)))

(fn ConstructionScript)

(fn SoundSequenceVerification
  (params (MusicKeyReferences :type BP%20Music%20Key%20Object%20Reference))
  (for (_array_element _array_index) (Variables|Default|GetMusicKeyReferences)
    (Development|PrintString (Utilities|GetDisplayName _array_element))
    (if (== _array_element MusicKeyReferences)
      (if (== _array_index (Variables|Default|GetSequenceCounter))
        (if (== (Variables|Default|GetSequenceCounter) (- (Utilities|Array|Length (Variables|Default|GetMusicKeyReferences)) 1))
          (Development|PrintString "Enigma Finished")
          (else
            (Math|Integer|IncrementInt (Variables|Default|GetSequenceCounter))))
        (else
          ;[1 1 1] Add some kind of feedback
          (Variables|Default|SetSequenceCounter 0))))))