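; Music puzzle slider that the player interacts with to cycle through music snippets.
; Box overlap shows and removes an interact prompt widget for the main character.
; Each interaction advances a wrapping index, plays the matching snippet and resets the character's movement.
; The mesh steps along a range split evenly at BeginPlay, jumping back to the start when the next step would reach the end.
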(event OnComponentBeginOverlap(Box)
  (params (OverlappedComponent :type Primitive%20Component%20Object%20Reference) (OtherActor :type Actor%20Object%20Reference) (OtherComp :type Primitive%20Component%20Object%20Reference) (OtherBodyIndex :type Integer) (bFromSweep :type Boolean) (SweepResult :type Hit%20Result%20Structure%20%28by%20ref%29))
  ;[1 1 1] Interact prompt
  (Utilities|Casting|CastToBP_MainCharacter OtherActor)
  (bind _returnvalue (UserInterface|CreateWidget "/Game/UI/BP_WGT_Interact.BP_WGT_Interact_C" (Game|GetPlayerController 0)))
  (bind _output_get (Variables|Default|SetInteractPrompt _returnvalue))
  (UserInterface|Viewport|AddtoViewport _output_get 0))

(event OnComponentEndOverlap(Box)
  (params (OverlappedComponent :type Primitive%20Component%20Object%20Reference) (OtherActor :type Actor%20Object%20Reference) (OtherComp :type Primitive%20Component%20Object%20Reference) (OtherBodyIndex :type Integer))
  ;[1 1 1] Interact prompt
  (Utilities|Casting|CastToBP_MainCharacter OtherActor)
  (Widget|RemovefromParent (Variables|Default|GetInteractPrompt)))

(event Custom|SliderPositionManager
  (bind _slidermovementincrement (Variables|SliderMovement|GetsliderMovementIncrement))
  (bind _slidermovementrange (Variables|SliderMovement|GetsliderMovementRange))
  (bind _staticmesh (Variables|Default|GetStaticMesh))
  (bind _relativelocation (Variables|/Script/Engine.SceneComponent|GetRelativeLocation _staticmesh))
  (bind _returnvalue (+ _relativelocation _slidermovementincrement))
  ;[1 1 1] Slider position manager
  (if (Math|Vector|Equal(Vector) _returnvalue (Utilities|Array|Get(acopy) _slidermovementrange 1) 1e-05)
    (Transformation|SetRelativeLocation _staticmesh (Utilities|Array|Get(acopy) _slidermovementrange) false false)
    (else
      (Transformation|SetRelativeLocation _staticmesh _returnvalue false false))))

(event EventInteract
  (params (FromEnigma? :type Boolean))
  (bind _audio (Variables|Default|GetAudio))
  ;[1 1 1] Interact
  (Audio|Components|Audio|Stop (Variables|Default|GetAudio))
  (bind _result (Math|Integer|IncrementInt (Variables|sliderLogic|GetSliderPosition))
    (:%20%20
      (if (== _result (Variables|sliderLogic|GetMaxSliderPosition))
        (Variables|sliderLogic|SetSliderPosition 0))
      (Audio|Components|Audio|SetSound _audio (Utilities|Array|Get(acopy) (Variables|Music|GetMusicSnipet) (Variables|sliderLogic|GetSliderPosition)))
      (Audio|Components|Audio|Play _audio 0.0)
      (CallFunction|SliderPositionManager)
      (bind _asbp_main_character (Utilities|Casting|CastToBP_MainCharacter (Game|GetPlayerCharacter 0)))
      (Default|ResetMovement _asbp_main_character))))

(event EventBeginPlay
  (bind _slidermovementrange (Variables|SliderMovement|GetsliderMovementRange))
  ;[1 1 1] Slider position manager
  (Transformation|SetRelativeLocation (Variables|Default|GetStaticMesh) (Utilities|Array|Get(acopy) (Variables|SliderMovement|GetsliderMovementRange)) false false)
  (Variables|SliderMovement|SetsliderMovementIncrement (/ (- (Utilities|Array|Get(acopy) _slidermovementrange 1) (Utilities|Array|Get(acopy) _slidermovementrange)) (Variables|sliderLogic|GetMaxSliderPosition))))

(fn ConstructionScript)