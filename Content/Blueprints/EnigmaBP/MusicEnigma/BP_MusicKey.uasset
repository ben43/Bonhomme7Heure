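; BP_MusicKey is an interactable key in the music enigma that plays a sound as part of a sequence puzzle.
; Its Box overlap with BP_MainCharacter shows or removes a BP_WGT_Interact prompt and toggles CanInteract.
; When PlayerInteractionAttempt fires while CanInteract is set, it plays its Audio and passes itself to BP_MusicMaster's SoundSequenceVerification, finding that actor by class.
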(event OnComponentBeginOverlap(Box)
  (params (OverlappedComponent :type Primitive%20Component%20Object%20Reference) (OtherActor :type Actor%20Object%20Reference) (OtherComp :type Primitive%20Component%20Object%20Reference) (OtherBodyIndex :type Integer) (bFromSweep :type Boolean) (SweepResult :type Hit%20Result%20Structure%20%28by%20ref%29))
  (Utilities|Casting|CastToBP_MainCharacter OtherActor)
  (bind _returnvalue (UserInterface|CreateWidget "/Game/UI/BP_WGT_Interact.BP_WGT_Interact_C" (Game|GetPlayerController 0)))
  (bind _output_get (Variables|Default|SetInteractPrompt _returnvalue))
  (UserInterface|Viewport|AddtoViewport _output_get 0)
  (Variables|Default|SetCanInteract true))

(event OnComponentEndOverlap(Box)
  (params (OverlappedComponent :type Primitive%20Component%20Object%20Reference) (OtherActor :type Actor%20Object%20Reference) (OtherComp :type Primitive%20Component%20Object%20Reference) (OtherBodyIndex :type Integer))
  (Utilities|Casting|CastToBP_MainCharacter OtherActor)
  (Widget|RemovefromParent (Variables|Default|GetInteractPrompt))
  (Variables|Default|SetCanInteract false))

(event Custom|PlayerInteractionAttempt
  (if (Variables|Default|GetCanInteract)
    (bind _returnvalue (Actor|GetActorOfClass "/Game/Blueprints/EnigmaBP/MusicEnigma/BP_MusicMaster.BP_MusicMaster_C"))
    (Audio|Components|Audio|Play (Variables|Default|GetAudio) 0.0)
    (Default|SoundSequenceVerification _returnvalue self)))

(event EventBeginPlay)

(event Collision|EventActorBeginOverlap
  (params (OtherActor :type Actor%20Object%20Reference)))

(event EventTick
  (params (DeltaSeconds :type Float%20%28single-precision%29)))

(fn ConstructionScript)