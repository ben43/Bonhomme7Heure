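; BP_Symbol is an interactable enigma symbol that completes a puzzle when the player interacts with it.
; Interact resets the main character's movement, spawns a pickup particle effect at the mesh location and destroys the static mesh component, leaving the actor itself in place.
; It then plays a success sound and calls EnigmaFinishedTrigger on the BP_ProgressionManager found in the level.
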(event EventBeginPlay)

(event Collision|EventActorBeginOverlap
  (params (OtherActor :type Actor%20Object%20Reference)))

(event EventTick
  (params (DeltaSeconds :type Float%20%28single-precision%29)))

(event EventInteract
  (params (FromEnigma? :type Boolean))
  (bind _asbp_main_character (Utilities|Casting|CastToBP_MainCharacter (Game|GetPlayerCharacter 0)))
  (Default|ResetMovement _asbp_main_character)
  (Effects|SpawnEmitteratLocation "/Game/VFX/P_ItemPickup.P_ItemPickup" (Transformation|GetWorldLocation (Variables|Default|GetStaticMesh)))
  (Components|DestroyComponent (Variables|Default|GetStaticMesh))
  (bind _returnvalue (Actor|GetActorOfClass "/Game/Blueprints/BP_ProgressionManager.BP_ProgressionManager_C"))
  (Audio|PlaySound2D "/Game/Sounds/SFX/Enigmas/Engma_Success01.Engma_Success01" 1.0 1.0 0.0 0 0)
  (Default|EnigmaFinishedTrigger _returnvalue))

(fn ConstructionScript)