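; BP_Fetch_Master runs a fetch puzzle (enigma) that is solved when the required BP_Fetch_Objects are inside its Box volume.
; Box overlap events raise or lower a found counter for actors listed in Objects.
; When the count reaches the list length, it triggers the level's BP_ProgressionManager, sends InteractMessage to Interactable and plays a success sound.
; BeginPlay locates that manager and prints a warning if none exists.
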(event OnComponentBeginOverlap(Box)
  (params (OverlappedComponent :type Primitive%20Component%20Object%20Reference) (OtherActor :type Actor%20Object%20Reference) (OtherComp :type Primitive%20Component%20Object%20Reference) (OtherBodyIndex :type Integer) (bFromSweep :type Boolean) (SweepResult :type Hit%20Result%20Structure%20%28by%20ref%29))
  (bind _asbp_fetch_objects (Utilities|Casting|CastToBP_Fetch_Objects OtherActor))
  (if (Utilities|Array|ContainsItem (Variables|RequiredOption|GetObjects) _asbp_fetch_objects)
    (bind _result (Math|Integer|IncrementInt (Variables|Default|GetObjectFound))
      (:%20%20
        (Development|PrintString (Utilities|String|ToString(Integer) _result))
        (if (== _result (Utilities|Array|Length (Variables|RequiredOption|GetObjects)))
          (Default|EnigmaFinishedTrigger (Variables|Default|GetProgressionManager))
          (Class|BPiInteract|Interact(Message) (Variables|EnigmaResolved(MANDATORY)|GetInteractable))
          (Audio|PlaySound2D "/Game/Sounds/SFX/Enigmas/Engma_Success01.Engma_Success01" 2.0 1.0 0.0 0 0))))))

(event OnComponentEndOverlap(Box)
  (params (OverlappedComponent :type Primitive%20Component%20Object%20Reference) (OtherActor :type Actor%20Object%20Reference) (OtherComp :type Primitive%20Component%20Object%20Reference) (OtherBodyIndex :type Integer))
  (bind _asbp_fetch_objects (Utilities|Casting|CastToBP_Fetch_Objects OtherActor))
  (if (Utilities|Array|ContainsItem (Variables|RequiredOption|GetObjects) _asbp_fetch_objects)
    (Math|Integer|DecrementInt (Variables|Default|GetObjectFound))))

(event EventBeginPlay
  (bind _returnvalue (Actor|GetActorOfClass "/Game/Blueprints/BP_ProgressionManager.BP_ProgressionManager_C"))
  (bind _output_get (Variables|Default|SetProgressionManager _returnvalue))
  (if (== _output_get 0)
    (Development|PrintString "No progression master in the level, pls insert one in order to make the game winnable" true true "(R=1.000000,G=0.018730,B=0.881678,A=1.000000)" 1e+01)))

(fn ConstructionScript)