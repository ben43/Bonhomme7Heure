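; BP_Radio is an interactable puzzle radio that, once powered, toggles static on and off with each interaction.
; With an object found, switching on also plays the tape song, and the first time closes the door and notifies BP_ProgressionManager after a delay that the enigma is finished.
; The first interaction opens the tape door, independent of power, with timelines animating its rotation.
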(event Custom|CloseRadioDoor
  (bind _door (Variables|Default|GetDoor))
  ;[1 1 1] Close the door
  (Audio|SpawnSoundatLocation "/Game/Sounds/SFX/Radio/RadioTapeDeck_Close.RadioTapeDeck_Close" (Transformation|GetWorldLocation _door) "0, 0, 0" 1.0 1.0 0.0 "/Game/Sounds/Attenuations/Footstep.Footstep" 0)
  (bind _alpha (Timeline|Timeline_1 Play)
    (:Update
      (Transformation|SetRelativeRotation _door (Math|Rotator|Lerp(Rotator) (Variables|/Script/Engine.SceneComponent|GetRelativeRotation _door) "0, 0, 0" _alpha) false false))))

(event Custom|OpenRadioDoor
  (bind _door (Variables|Default|GetDoor))
  ;[1 1 1] Opens the door
  (Utilities|FlowControl|DoOnce false
    (:Completed
      (Audio|SpawnSoundatLocation "/Game/Sounds/SFX/Radio/RadioTapeDeck_Close.RadioTapeDeck_Close" (Transformation|GetWorldLocation _door) "0, 0, 0" 1.0 1.0 0.0 "/Game/Sounds/Attenuations/Footstep.Footstep" 0)
      (bind _alpha (Timeline|Timeline_0 Play)
        (:Update
          (Transformation|SetRelativeRotation _door (Math|Rotator|Lerp(Rotator) (Variables|/Script/Engine.SceneComponent|GetRelativeRotation _door) (Variables|Default|GetDoorRotationAmount) _alpha) false false))))))

(event EventBeginPlay
  (|CallParentFunction) ; This node is disabled and will not be called.\nDrag off pins to build functionality.
)

(event EventInteract
  (params (FromEnigma? :type Boolean))
  (bind _returnvalue (Transformation|GetActorLocation))
  (if (Variables|Default|GetCanInteractWith?)
    (bind _asbp_main_character (Utilities|Casting|CastToBP_MainCharacter (Game|GetPlayerCharacter 0)))
    (Default|ResetMovement _asbp_main_character)
    (Audio|SpawnSoundatLocation (Variables|Default|GetAudioOnInteract) _returnvalue "0, 0, 0" 1.0 1.0 0.0 "/Game/Sounds/Attenuations/Footstep.Footstep" 0)
    (Utilities|FlowControl|Sequence
      (:then_0
        (if (Variables|Default|GetIsPowerOn?)
          (Utilities|FlowControl|FlipFlop
            (:A
              (bind _returnvalue_2 (Audio|SpawnSoundatLocation "/Game/Sounds/Cues/A_RadioStatic_Cue.A_RadioStatic_Cue" _returnvalue "0, 0, 0" 1.0 1.0 0.0 "/Game/Sounds/Attenuations/Footstep.Footstep" 0))
              (if (> (Variables|Default|GetObjectFound) 0)
                (Audio|SpawnSoundatLocation "/Game/Sounds/SFX/Radio/RadioTapeDeck_Play.RadioTapeDeck_Play" _returnvalue "0, 0, 0" 3.0 1.0 0.0 "/Game/Sounds/Attenuations/Footstep.Footstep" 0)
                (bind _returnvalue_3 (Audio|SpawnSoundatLocation (Variables|Default|GetRadioSong) _returnvalue "0, 0, 0" 3.0 1.0 0.0 "/Game/Sounds/Attenuations/Footstep.Footstep" 0))
                (Utilities|FlowControl|DoOnce false
                  (:Completed
                    (Utilities|FlowControl|Sequence
                      (:then_0
                        (Utilities|FlowControl|Delay 16.0)
                        (bind _returnvalue_4 (Actor|GetActorOfClass "/Game/Blueprints/BP_ProgressionManager.BP_ProgressionManager_C"))
                        (Default|EnigmaFinishedTrigger _returnvalue_4))
                      (:then_1
                        (CallFunction|CloseRadioDoor)))))))
            (:B
              (Components|DestroyComponent _returnvalue_3)))))
      (:then_1
        (CallFunction|OpenRadioDoor)))))

(event EventActivatePower
  (Variables|Default|SetIsPowerOn? true))

(event Collision|EventActorBeginOverlap
  (params (OtherActor :type Actor%20Object%20Reference)))

(event EventTick
  (params (DeltaSeconds :type Float%20%28single-precision%29)))

(fn ConstructionScript
  (|CallParentFunction))

(fn EndOverlap
  (params (Actor :type Actor%20Object%20Reference)))

(fn EndOfEnigma)