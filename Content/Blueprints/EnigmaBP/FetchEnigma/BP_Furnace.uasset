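; Puzzle furnace that consumes tagged items and spawns a symbol once it holds oil (Huile), wood (Bois) and cursed wood.
; Interacting while InRange slides the door once.
; The interior overlap reads actor tags to set item flags, plays a pickup effect and destroys the actor.
; Separately, Trigger ignites the fire once, provided ActivatePower has run and oil and wood are inside.
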(event OnComponentBeginOverlap(Box)
  (params (OverlappedComponent :type Primitive%20Component%20Object%20Reference) (OtherActor :type Actor%20Object%20Reference) (OtherComp :type Primitive%20Component%20Object%20Reference) (OtherBodyIndex :type Integer) (bFromSweep :type Boolean) (SweepResult :type Hit%20Result%20Structure%20%28by%20ref%29))
  (bind _asbp_main_character (Utilities|Casting|CastToBP_MainCharacter OtherActor))
  (Variables|Default|SetPlayerRef _asbp_main_character))

(event OnComponentEndOverlap(Box)
  (params (OverlappedComponent :type Primitive%20Component%20Object%20Reference) (OtherActor :type Actor%20Object%20Reference) (OtherComp :type Primitive%20Component%20Object%20Reference) (OtherBodyIndex :type Integer))
  (if (== OtherActor (Variables|Default|GetPlayerRef))
    _))

(event OnComponentBeginOverlap(Interior)
  (params (OverlappedComponent :type Primitive%20Component%20Object%20Reference) (OtherActor :type Actor%20Object%20Reference) (OtherComp :type Primitive%20Component%20Object%20Reference) (OtherBodyIndex :type Integer) (bFromSweep :type Boolean) (SweepResult :type Hit%20Result%20Structure%20%28by%20ref%29))
  (bind _array_element (Utilities|Array|ForEachLoopwithBreak (Variables|/Script/Engine.Actor|GetTags OtherActor))
    (:LoopBody
      ;[1 1 1] Check tags name
      (if (Utilities|Name|Equal(Name) _array_element "Huile")
        (Variables|Default|SetGotHuile (Utilities|Name|Equal(Name) _array_element "Huile"))
        (CallFunction|BreakLoop :!label _label)
        (elif (Utilities|Name|Equal(Name) _array_element "Bois")
          (Variables|Default|SetGotBois (Utilities|Name|Equal(Name) _array_element "Bois"))
          (goto _label)
          (elif (Utilities|Name|Equal(Name) _array_element "CursedWood")
            (Variables|Default|SetGotCursedWood (Utilities|Name|Equal(Name) _array_element "CursedWood"))
            (goto _label)))))
    (:Completed
      (bind _returnvalue (Effects|SpawnEmitteratLocation "/Game/VFX/P_ItemPickup.P_ItemPickup" (Transformation|GetWorldLocation OtherComp) "0, 0, 0" "2.000000,2.000000,2.000000"))
      (Variables|Default|SetFireParticles _returnvalue)
      ;[1 1 1] All objects in furnace?
      (Actor|DestroyActor OtherActor)
      (if (and (and (Variables|Default|GetGotHuile) (Variables|Default|GetGotBois)) (Variables|Default|GetGotCursedWood))
        (Development|PrintString "All Objects in furnace")
        ;[1 1 1] Spawn Symbol
        (Game|SpawnActorfromClass "/Game/Blueprints/EnigmaBP/BP_Symbol.BP_Symbol_C" (Math|Conversions|ToTransform(Vector) (+ (Transformation|GetActorLocation) "30.000000,70.000000,10.000000")) "Undefined" 0 0)
        (Components|DestroyComponent (Variables|Default|GetFireParticles))))))

(event Custom|BreakLoop
  (Utilities|Array|ForEachLoopwithBreak (Variables|/Script/Engine.Actor|GetTags (stale OnComponentBeginOverlap(Interior) OtherActor))) ; enters at Break
)

(event EventTrigger
  (params (Reference :type Actor%20Object%20Reference))
  (if (stale EventActivatePower _output_get)
    ;[1 1 1] Ignite Fire
    (if (and (Variables|Default|GetGotHuile) (Variables|Default|GetGotBois))
      (Utilities|FlowControl|DoOnce false
        (:Completed
          (Effects|SpawnEmitteratLocation "/Engine/Tutorial/SubEditors/TutorialAssets/TutorialParticleSystem.TutorialParticleSystem" (Transformation|GetWorldLocation (Variables|Default|GetSM_Furnace_Interior)) "0, 0, 0" "0.200000,0.200000,0.200000")
          (Variables|Default|SetFireIgnited? true))))))

(event Collision|EventActorBeginOverlap
  (params (OtherActor :type Actor%20Object%20Reference)))

(event EventTick
  (params (DeltaSeconds :type Float%20%28single-precision%29)))

(event EventInteract
  (params (FromEnigma? :type Boolean))
  (bind _asbp_main_character (Utilities|Casting|CastToBP_MainCharacter (Game|GetPlayerCharacter 0)))
  (Default|ResetMovement _asbp_main_character)
  (if (Variables|Default|GetInRange)
    ;[1 1 1] Move Door
    (Utilities|FlowControl|DoOnce false
      (:Completed
        (Transformation|AddLocalOffset (Variables|Default|GetSM_Furnace_Door) "30.000000,0.000000, 0" false false)))))

(event EventActivatePower
  (bind _output_get (Variables|Default|SetIsPowerOn? true)))

(fn ConstructionScript)