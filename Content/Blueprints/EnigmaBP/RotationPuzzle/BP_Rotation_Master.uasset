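; Master Blueprint for a rotation puzzle that notifies the progression manager and unlocks a reward safe when solved.
; BeginPlay finds the level's BP_ProgressionManager, printing a warning if missing.
; Box overlaps flag the main character's proximity, gating a one-second delayed loop in TickEvent.
; The loop compares Child's pitch to its own ±10 degrees, joining both bounds with OR, with no completion guard.
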(event OnComponentBeginOverlap(Box)
  (params (OverlappedComponent :type Primitive%20Component%20Object%20Reference) (OtherActor :type Actor%20Object%20Reference) (OtherComp :type Primitive%20Component%20Object%20Reference) (OtherBodyIndex :type Integer) (bFromSweep :type Boolean) (SweepResult :type Hit%20Result%20Structure%20%28by%20ref%29))
  (Utilities|Casting|CastToBP_MainCharacter OtherActor)
  (Variables|Default|SetPlayerClose true))

(event OnComponentEndOverlap(Box)
  (params (OverlappedComponent :type Primitive%20Component%20Object%20Reference) (OtherActor :type Actor%20Object%20Reference) (OtherComp :type Primitive%20Component%20Object%20Reference) (OtherBodyIndex :type Integer))
  (Utilities|Casting|CastToBP_MainCharacter OtherActor)
  (Variables|Default|SetPlayerClose false))

(event Custom|TickEvent
  (bind _returnvalue (Transformation|GetActorRotation))
  (bind _child (Variables|RequiredOption|GetChild))
  (bind _returnvalue_2 (Transformation|GetActorRotation _child))
  (bind _returnvalue_3 (Math|Float|%(Float) (.pitch _returnvalue_2) 3.6e+02))
  (Utilities|WhileLoopwithDelay (Variables|Default|GetPlayerClose) 1.0
    (:LoopBody
      (if (or (<= _returnvalue_3 (Math|Float|%(Float) (+ (.pitch _returnvalue) 1e+01) 3.6e+02)) (>= _returnvalue_3 (Math|Float|%(Float) (- (.pitch _returnvalue) 1e+01) 3.6e+02)))
        (Default|EnigmaFinishedTrigger (Variables|Default|GetProgressionManager))
        (Default|SafeDoorUnlock (Variables|EnigmaResolved(MANDATORY)|GetRewardBox))))))

(event EventBeginPlay
  (bind _returnvalue (Actor|GetActorOfClass "/Game/Blueprints/BP_ProgressionManager.BP_ProgressionManager_C"))
  (bind _output_get (Variables|Default|SetProgressionManager _returnvalue))
  (if (== _output_get 0)
    (Development|PrintString "No progression master in the level, pls insert one in order to make the game winnable" true true "(R=1.000000,G=0.018730,B=0.881678,A=1.000000)" 1e+01)))

(fn ConstructionScript)