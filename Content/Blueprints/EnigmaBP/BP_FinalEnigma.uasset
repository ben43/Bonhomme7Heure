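; Final enigma actor that shows an interact prompt when the main character enters its box.
; Interact checks the progression manager: a positive EnigmaFinished count plays a success sound and forwards the interaction to a linked Interactable.
; Otherwise, if in range, it halts the player and fades to a clock camera for a timed look before restoring view and control.
; During that view, the EnigmasFinished flag gates the last-enigma UI.
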(event OnComponentBeginOverlap(Box)
  (params (OverlappedComponent :type Primitive%20Component%20Object%20Reference) (OtherActor :type Actor%20Object%20Reference) (OtherComp :type Primitive%20Component%20Object%20Reference) (OtherBodyIndex :type Integer) (bFromSweep :type Boolean) (SweepResult :type Hit%20Result%20Structure%20%28by%20ref%29))
  (Utilities|Casting|CastToBP_MainCharacter OtherActor)
  (bind _returnvalue (UserInterface|CreateWidget "/Game/UI/BP_WGT_Interact.BP_WGT_Interact_C"))
  (bind _output_get (Variables|Default|SetInteractPrompt _returnvalue))
  (UserInterface|Viewport|AddtoViewport _output_get 0)
  (Variables|Default|SetPlayerInRange true))

(event OnComponentEndOverlap(Box)
  (params (OverlappedComponent :type Primitive%20Component%20Object%20Reference) (OtherActor :type Actor%20Object%20Reference) (OtherComp :type Primitive%20Component%20Object%20Reference) (OtherBodyIndex :type Integer))
  (Utilities|Casting|CastToBP_MainCharacter OtherActor)
  (Widget|RemovefromParent (Variables|Default|GetInteractPrompt))
  (Variables|Default|SetPlayerInRange false))

(event Custom|SpendSymbol
  ;[1 1 1] Spending a Symbol
  (Audio|SpawnSound2D "/Game/Sounds/SFX/Enigmas/Engma_Success01.Engma_Success01" 1.0 1.0 0.0 0)
  (bind _output_get (Variables|Default|SetFromEnigma? true))
  (Default|Interact (Variables|Default|GetInteractable) _output_get))

(event Custom|GetClockCamera
  (bind _returnvalue (Game|GetPlayerCameraManager 0))
  ;[1 1 1] Blend Into camera and wait
  (CameraFades|StartCameraFade :self _returnvalue :FromAlpha 1.0 :Duration (Variables|Default|GetFadeDuration))
  (Game|Player|SetViewTargetwithBlend (Game|GetPlayerController 0) (Variables|Default|GetCameraRef) 3.0 "VTBlend_Cubic" 0.0 false)
  (if (Variables|Default|GetEnigmasFinished)
    (CallFunction|DisplayUi 2.0))
  (Utilities|FlowControl|Delay (Variables|Default|GetReadTime))
  (CameraFades|StartCameraFade :self _returnvalue :ToAlpha 1.0 :Duration (Variables|Default|GetFadeDuration))
  (CallFunction|GetPlayerCamera))

(event Custom|GetPlayerCamera
  (bind _returnvalue (Game|GetPlayerController 0))
  ;[1 1 1] Get back into Player's camera
  (Utilities|FlowControl|Delay (Variables|Default|GetFadeDuration))
  (Game|Player|SetViewTargetwithBlend _returnvalue (Variables|Default|GetPlayerCamera) 0.0 "VTBlend_Linear" 0.0 false)
  (CameraFades|StartCameraFade :self (Game|GetPlayerCameraManager 0) :FromAlpha 1.0 :Duration (Variables|Default|GetFadeDuration))
  (Input|SetInputModeGameOnly _returnvalue)
  (Components|Activation|Activate (Pawn|GetMovementComponent (Game|GetPlayerCharacter 0)) true))

(event Custom|DisplayUi
  (params (WaitBeforeTime :type Float%20%28single-precision%29))
  (bind _interactprompt (Variables|Default|GetInteractPrompt))
  ;[1 1 1] DisplayUi
  (Utilities|FlowControl|Delay WaitBeforeTime)
  (if (Variables|Default|GetEnigmasFinished)
    (Widget|RemovefromParent _interactprompt)
    (bind _returnvalue (UserInterface|CreateWidget "/Game/UI/BP_WGT_LastEnigma.BP_WGT_LastEnigma_C"))
    (bind _output_get (Variables|Default|SetEnigmaUI _returnvalue))
    (UserInterface|Viewport|AddtoViewport _output_get 0)
    (else
      (Widget|RemovefromParent _interactprompt)
      (bind _returnvalue_2 (UserInterface|CreateWidget "/Game/UI/BP_WGT_EnigmaNotFinished.BP_WGT_EnigmaNotFinished_C"))
      (bind _output_get_2 (Variables|Default|SetEnigmaNotFinishedPrompt _returnvalue_2))
      (UserInterface|Viewport|AddtoViewport _output_get_2 0)
      (Utilities|FlowControl|Delay 3.0)
      (Widget|RemovefromParent _output_get_2))))

(event EventInteract
  (params (FromEnigma? :type Boolean))
  (bind _returnvalue (Game|GetPlayerController 0))
  (if (> (Variables|/Game/Blueprints/BP_ProgressionManager.BP_ProgressionManager_C|GetEnigmaFinished (Variables|Default|GetProgressionManagerRef)) 0)
    (CallFunction|SpendSymbol)
    (elif (Variables|Default|GetPlayerInRange)
      (Widget|RemovefromParent (Variables|Default|GetInteractPrompt))
      (Components|Activation|Deactivate (Pawn|GetMovementComponent (Game|GetPlayerCharacter 0)))
      ;[1 1 1] Fadeout, Set input Ui only
      (Variables|Default|SetPlayerCamera (Pawn|GetViewTarget _returnvalue))
      (Input|SetInputModeUIOnly _returnvalue 0 "DoNotLock")
      (CameraFades|StartCameraFade :self (Game|GetPlayerCameraManager 0) :ToAlpha 1.0 :Duration (Variables|Default|GetFadeDuration) :bHoldWhenFinished true)
      (Utilities|FlowControl|Delay (Variables|Default|GetFadeDuration))
      (CallFunction|GetClockCamera))))

(event EventBeginPlay
  ;[1 1 1] Get ProgressionManager Ref
  (bind _outactors (Actor|GetAllActorsOfClass "/Game/Blueprints/BP_ProgressionManager.BP_ProgressionManager_C"))
  (Variables|Default|SetProgressionManagerRef (Utilities|Array|Get(acopy) _outactors)))

(fn ConstructionScript)