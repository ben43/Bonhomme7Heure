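; BP_HideNSeek_Master is the master Blueprint for a find-and-seek puzzle, tracking how many objects have been found.
; BeginPlay caches the level's BP_ProgressionManager, with a printed warning for a missing one.
; ObjectFoundUpdate increments the count; when it equals the ObjectToFind list length, it notifies the progression manager that the enigma is finished and unlocks the RewardBox safe door.
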(event EventBeginPlay
  (bind _returnvalue (Actor|GetActorOfClass "/Game/Blueprints/BP_ProgressionManager.BP_ProgressionManager_C"))
  (bind _output_get (Variables|Default|SetProgressionManager _returnvalue))
  (if (== _output_get 0)
    (Development|PrintString "No progression master in the level, pls insert one in order to make the game winnable" true true "(R=1.000000,G=0.018730,B=0.881678,A=1.000000)" 1e+01)))

(fn ConstructionScript)

(fn ObjectFoundUpdate
  (Variables|Default|SetObjectFound (+ (Variables|Default|GetObjectFound) 1))
  (if (== (Variables|Default|GetObjectFound) (Utilities|Array|Length (Variables|RequiredOption|GetObjectToFind)))
    ;[1 1 1] UnlockThingy+PlayMusic
    (Default|EnigmaFinishedTrigger (Variables|Default|GetProgressionManager))
    (Default|SafeDoorUnlock (Variables|EnigmaResolved(MANDATORY)|GetRewardBox))))