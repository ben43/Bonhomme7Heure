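; Interactable safe puzzle: the child character opens its enigma widget, while the adult only triggers a dad voice line with the music ducked.
; Box overlaps track reach and which character is present, showing an interact prompt.
; Once EnigmaDone is set, interacting collects the symbol with particles and sound, then notifies BP_ProgressionManager.
; OpenDoor, not called within this graph, swings the door open on a delayed timeline with a positional sound.
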(event OnComponentBeginOverlap(Box)
  (params (OverlappedComponent :type Primitive%20Component%20Object%20Reference) (OtherActor :type Actor%20Object%20Reference) (OtherComp :type Primitive%20Component%20Object%20Reference) (OtherBodyIndex :type Integer) (bFromSweep :type Boolean) (SweepResult :type Hit%20Result%20Structure%20%28by%20ref%29))
  (Utilities|Casting|CastToBP_ChildCharacter OtherActor
    (:then
      (bind _returnvalue (UserInterface|CreateWidget "/Game/UI/BP_WGT_Interact.BP_WGT_Interact_C"))
      (bind _output_get (Variables|Default|SetInteract_Widget _returnvalue))
      (UserInterface|Viewport|AddtoViewport _output_get 0)
      (Variables|Default|SetplayerInReach true))
    (:CastFailed
      (Utilities|Casting|CastToBP_AdultCharacter OtherActor)
      (Variables|Default|SetIsDad? true)
      (bind _returnvalue_2 (UserInterface|CreateWidget "/Game/UI/BP_WGT_Interact.BP_WGT_Interact_C"))
      (bind _output_get_2 (Variables|Default|SetInteract_Widget _returnvalue_2))
      (UserInterface|Viewport|AddtoViewport _output_get_2 0)
      (Variables|Default|SetplayerInReach true))))

(event OnComponentEndOverlap(Box)
  (params (OverlappedComponent :type Primitive%20Component%20Object%20Reference) (OtherActor :type Actor%20Object%20Reference) (OtherComp :type Primitive%20Component%20Object%20Reference) (OtherBodyIndex :type Integer))
  (Utilities|Casting|CastToBP_ChildCharacter OtherActor
    (:then
      (Widget|RemovefromParent (Variables|Default|GetInteract_Widget))
      (Variables|Default|SetplayerInReach false))
    (:CastFailed
      (Utilities|Casting|CastToBP_AdultCharacter OtherActor)
      (Variables|Default|SetIsDad? false)
      (Widget|RemovefromParent (Variables|Default|GetInteract_Widget))
      (Variables|Default|SetplayerInReach false))))

(event Custom|OnAudioFinished_DadLine
  ;[1 1 1] Audio Dadline
  (Audio|SetSoundMixClassOverride "/Game/Sounds/SoundsClasses/B7H_SCM_Master.B7H_SCM_Master" "/Game/Sounds/SoundsClasses/B7H_Music.B7H_Music" 1.0 1.0 1.0 true)
  (CallFunction|ResetDadLine)
  (Default|ResetMovement (Variables|Default|GetPlayerRef))
  (Default|ResetMovement (Variables|Default|GetPlayerRef))
  (bind _returnvalue (UserInterface|CreateWidget "/Game/UI/BP_WGT_Crosshair.BP_WGT_Crosshair_C" (Game|GetPlayerController 0)))
  (UserInterface|Viewport|AddtoViewport _returnvalue 0))

(event Custom|OpenDoor
  (bind _sm_safe_door (Variables|Default|GetSM_Safe_Door))
  ;[1 1 1] Opens the door
  (Utilities|FlowControl|Delay 1.0)
  (bind _alpha (Timeline|OpensDoor Play)
    (:Update
      (Transformation|SetRelativeRotation _sm_safe_door (Math|Rotator|Lerp(Rotator) (Variables|/Script/Engine.SceneComponent|GetRelativeRotation _sm_safe_door) (Variables|Default|GetDoorRotationAmount) _alpha) false false)
      (Utilities|FlowControl|DoOnce false
        (:Completed
          (Audio|SpawnSoundatLocation "/Game/Sounds/SFX/Safe/A_SafeOpening.A_SafeOpening" (Transformation|GetWorldLocation _sm_safe_door) "0, 0, 0" 3.0 1.0 0.0 "/Game/Sounds/Attenuations/Footstep.Footstep" 0))))))

(event Custom|ResetDadLine
  ;[1 1 1] Audio Dadline
  (Utilities|FlowControl|DoOnce false) ; enters at Reset
)

(event EventBeginPlay
  (bind _outactors (Actor|GetAllActorsOfClass "/Game/Blueprints/BP_ProgressionManager.BP_ProgressionManager_C"))
  (Variables|Default|SetProgressionManager (Utilities|Array|Get(acopy) _outactors)))

(event EventInteract
  (params (FromEnigma? :type Boolean))
  (bind _returnvalue (Game|GetPlayerController 0))
  (bind _symbolmesh (Variables|Default|GetSymbolMesh))
  (bind _asbp_main_character (Utilities|Casting|CastToBP_MainCharacter (Game|GetPlayerCharacter 0)))
  (Variables|Default|SetPlayerRef _asbp_main_character)
  (Default|ResetMovement (Variables|Default|GetPlayerRef))
  (if (Variables|Default|GetplayerInReach)
    (Viewport|RemoveAllWidgets)
    (if (Variables|Default|GetEnigmaDone?)
      (Utilities|FlowControl|DoOnce false
        (:Completed
          (Effects|SpawnEmitteratLocation (Variables|Default|GetParticlesSpawn) (Transformation|GetWorldLocation _symbolmesh))
          (Components|DestroyComponent _symbolmesh)
          ;[1 1 1] Finishing Enigma
          (bind _returnvalue_2 (Actor|GetActorOfClass "/Game/Blueprints/BP_ProgressionManager.BP_ProgressionManager_C"))
          (Audio|PlaySound2D "/Game/Sounds/SFX/Enigmas/Engma_Success01.Engma_Success01" 1.0 1.0 0.0 0 0)
          (Default|EnigmaFinishedTrigger _returnvalue_2)
          (Default|ResetMovement (Variables|Default|GetPlayerRef))
          (bind _returnvalue_3 (UserInterface|CreateWidget "/Game/UI/BP_WGT_Crosshair.BP_WGT_Crosshair_C" (Game|GetPlayerController 0)))
          (UserInterface|Viewport|AddtoViewport _returnvalue_3 0)))
      (elif (Variables|Default|GetIsDad?)
        ;[1 1 1] Audio Dadline
        (Default|ResetMovement (Variables|Default|GetPlayerRef))
        (Utilities|FlowControl|DoOnce false
          (:Completed
            (Audio|SetSoundMixClassOverride "/Game/Sounds/SoundsClasses/B7H_SCM_Master.B7H_SCM_Master" "/Game/Sounds/SoundsClasses/B7H_Music.B7H_Music" 0.3 1.0 1.0 true)
            (bind _returnvalue_4 (Audio|CreateSound2D (Variables|Default|GetDad%20Line) 0.5 1.0 0.0 0))
            (Audio|Components|Audio|Play _returnvalue_4 0.0)
            (EventDispatchers|AssignOnAudioFinished _returnvalue_4 (delegate Custom|OnAudioFinished_DadLine))))
        (else
          ;[1 1 1] Display Widget Enigma
          (bind _returnvalue_5 (UserInterface|CreateWidget "/Game/UI/BP_WGT_CoffreFortEnigma.BP_WGT_CoffreFortEnigma_C"))
          (UserInterface|Viewport|AddtoViewport _returnvalue_5 0)
          (Input|SetInputModeUIOnly _returnvalue 0 "DoNotLock")
          (Variables|/Script/Engine.PlayerController|SetbShowMouseCursor _returnvalue true))))))

(fn ConstructionScript)