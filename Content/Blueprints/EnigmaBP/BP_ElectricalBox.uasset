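; BP_ElectricalBox is an interactable electrical box that switches on power for the level, likely as a puzzle step.
; It caches all BPi_Interact actors on BeginPlay and shows an interact widget while the main character is inside its box trigger.
; Interact resets player movement, then a DoOnce sends ActivatePowerMessage to every cached actor, rotates the handle, and plays power-on sounds and a particle effect.
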(event OnComponentBeginOverlap(Box)
  (params (OverlappedComponent :type Primitive%20Component%20Object%20Reference) (OtherActor :type Actor%20Object%20Reference) (OtherComp :type Primitive%20Component%20Object%20Reference) (OtherBodyIndex :type Integer) (bFromSweep :type Boolean) (SweepResult :type Hit%20Result%20Structure%20%28by%20ref%29))
  (Utilities|Casting|CastToBP_MainCharacter OtherActor)
  (bind _returnvalue (UserInterface|CreateWidget "/Game/UI/BP_WGT_Interact.BP_WGT_Interact_C"))
  (bind _output_get (Variables|Default|SetInteractUi _returnvalue))
  (UserInterface|Viewport|AddtoViewport _output_get 0)
  (Variables|Default|SetInRange? true))

(event OnComponentEndOverlap(Box)
  (params (OverlappedComponent :type Primitive%20Component%20Object%20Reference) (OtherActor :type Actor%20Object%20Reference) (OtherComp :type Primitive%20Component%20Object%20Reference) (OtherBodyIndex :type Integer))
  (Utilities|Casting|CastToBP_MainCharacter OtherActor)
  (Widget|RemovefromParent (Variables|Default|GetInteractUi))
  (Variables|Default|SetInRange? false))

(event EventBeginPlay
  (bind _outactors (Actor|GetAllActorswithInterface "/Game/Blueprints/BPi_Interact.BPi_Interact_C"))
  (Variables|Default|SetPowerableActors _outactors))

(event EventInteract
  (params (FromEnigma? :type Boolean))
  (bind _staticmesh (Variables|Default|GetStaticMesh))
  (bind _returnvalue (Transformation|GetWorldLocation _staticmesh))
  (bind _asbp_main_character (Utilities|Casting|CastToBP_MainCharacter (Game|GetPlayerCharacter 0)))
  (Default|ResetMovement _asbp_main_character)
  (Utilities|FlowControl|DoOnce false
    (:Completed
      (Utilities|FlowControl|Sequence
        (:then_0
          (for _array_element (Variables|Default|GetPowerableActors)
            (Class|BPiInteract|ActivatePower(Message) _array_element)))
        (:then_1
          (Transformation|SetRelativeRotation (Variables|Default|GetStaticMeshHandle) (Variables|Default|GetHandleRotation) false false)
          (CallFunction|PlayAudio _returnvalue)
          (Effects|SpawnEmitteratLocation "/Game/VFX/P_ItemPickup.P_ItemPickup" (+ _returnvalue "0,20.000000,10.000000") "0, 0, 0" "4.000000,4.000000,4.000000"))))))

(fn ConstructionScript)

(fn PlayAudio
  (params (Location :type Vector))
  (Audio|SpawnSoundatLocation "/Game/Sounds/SFX/PowerBox/PowerOn.PowerOn" Location "0, 0, 0" 3.0 1.0 0.0 "/Game/Sounds/Attenuations/Footstep.Footstep" 0)
  (Audio|SpawnSound2D "/Game/Sounds/SFX/Enigmas/Engma_Success01.Engma_Success01" 1.0 1.0 0.0 0)
  (Audio|SpawnSoundatLocation "/Game/Sounds/Cues/A_ElectricalHum_Cue.A_ElectricalHum_Cue" Location "0, 0, 0" 1.0 1.0 0.0 "/Game/Sounds/Attenuations/ElectricalHums.ElectricalHums" 0))