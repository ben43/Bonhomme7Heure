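; RandomEvents is a trigger actor that fires configurable events whenever BP_MainCharacter begins overlapping its Box.
; Boolean flags enable three independent branches: playing audio, teleporting the actor between two stored locations, and hiding or toggling its mesh.
; FlipFlops alternate location and visibility on successive overlaps.
; Sound stays locked for SoundDuration, then Repeat clears if 1TimeSound is false, opposite to what that name suggests.
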(event OnComponentBeginOverlap(Box)
  (params (OverlappedComponent :type Primitive%20Component%20Object%20Reference) (OtherActor :type Actor%20Object%20Reference) (OtherComp :type Primitive%20Component%20Object%20Reference) (OtherBodyIndex :type Integer) (bFromSweep :type Boolean) (SweepResult :type Hit%20Result%20Structure%20%28by%20ref%29))
  (bind _objectlocations (Variables|MoveObject|GetObjectLocations))
  (Utilities|Casting|CastToBP_MainCharacter OtherActor)
  (Utilities|FlowControl|Sequence
    (:then_0
      ;[1 1 1] SoundPlayed
      (if (Variables|Sound|GetSound?)
        (if (Variables|Sound|GetRepeat)
          (Audio|Components|Audio|Play (Variables|Default|GetAudio) 0.0)
          (Variables|Sound|SetSound? false)
          (Utilities|FlowControl|Delay (Variables|Sound|GetSoundDuration))
          (Variables|Sound|SetSound? true)
          (if (not (Variables|Sound|Get1TimeSound))
            (Variables|Sound|SetRepeat false)))))
    (:then_1
      ;[1 1 1] ObjectMove
      (if (Variables|MoveObject|GetObjectMove?)
        (Utilities|FlowControl|FlipFlop
          (:A
            (Transformation|SetActorLocation (Utilities|Array|Get(acopy) _objectlocations 1) false false))
          (:B
            (Transformation|SetActorLocation (Utilities|Array|Get(acopy) _objectlocations) false false)))))
    (:then_2
      ;[1 1 1] Object Disappear
      (if (Variables|ObjectDisapearrance|GetObjectDisapear?)
        (if (Variables|ObjectDisapearrance|GetObjectWillReappear?)
          (Utilities|FlowControl|FlipFlop
            (:A
              (Rendering|SetVisibility (Variables|Default|GetStaticMesh) false false))
            (:B
              (Rendering|SetVisibility (Variables|Default|GetStaticMesh) true false)))
          (else
            (Rendering|SetVisibility (Variables|Default|GetStaticMesh) false false)))))))

(fn ConstructionScript)