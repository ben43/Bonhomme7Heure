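; ProgressionManager is an actor that tracks how many enigmas the player has completed in the level.
; Shortly after BeginPlay, it counts all actors tagged "Enigma" to set the total.
; Each call to EnigmaFinishedTrigger increments a finished counter and prints a completion message once it reaches that total.
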(event EventBeginPlay
  (Utilities|FlowControl|Delay 0.2)
  (bind _outactors (Actor|GetAllActorswithTag "Enigma"))
  (Variables|Default|SetTotalNumberOfEnigma (Utilities|Array|Length _outactors)))

(event Collision|EventActorBeginOverlap
  (params (OtherActor :type Actor%20Object%20Reference)))

(event EventTick
  (params (DeltaSeconds :type Float%20%28single-precision%29)))

(fn ConstructionScript)

(fn EnigmaFinishedTrigger
  (bind _enigmafinished (Variables|Default|GetEnigmaFinished))
  (Math|Integer|IncrementInt _enigmafinished
    (:%20%20
      (if (>= _enigmafinished (Variables|Default|GetTotalNumberOfEnigma))
        (Development|PrintString "You've done all the enigma!")))))