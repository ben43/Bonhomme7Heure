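; BP_BreakableObject is a breakable prop, apparently a vase judging by its sound, that releases a key when it shatters.
; A StaticMesh hit above a speed threshold triggers a one-time swap to a spawned BP_Destructible, which is pushed downward and plays a breaking sound.
; It then spawns BP_Key at the destructible's location and passes it this object's DoorReference.
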(event OnComponentHit(StaticMesh)
  (params (HitComponent :type Primitive%20Component%20Object%20Reference) (OtherActor :type Actor%20Object%20Reference) (OtherComp :type Primitive%20Component%20Object%20Reference) (NormalImpulse :type Vector :default "0, 0, 0") (Hit :type Hit%20Result%20Structure%20%28by%20ref%29))
  (if (> (Math|Vector|VectorLength (Transformation|GetComponentVelocity (Variables|Default|GetStaticMesh))) 1.6e+02)
    (Utilities|FlowControl|DoOnce false
      (:Completed
        (Utilities|FlowControl|Sequence
          (:then_0
            (bind _returnvalue (Game|SpawnActorfromClass "/Game/Blueprints/BP_Destructible.BP_Destructible_C" (Transformation|GetWorldTransform (Variables|Default|GetStaticMesh)) "Undefined" 0 0))
            (Components|DestroyComponent (Variables|Default|GetStaticMesh))
            (Variables|Default|SetActorLocation (Transformation|GetActorLocation _returnvalue))
            (Physics|SetPhysicsLinearVelocity (Variables|/Game/Blueprints/BP_Destructible.BP_Destructible_C|GetDestructible _returnvalue) "0.000000,0.000000,-500.000000" false "None")
            (Audio|SpawnSoundatLocation "/Game/Sounds/SFX/Breaking/VaseBreaking.VaseBreaking" (Transformation|GetActorLocation _returnvalue) "0, 0, 0" 2.0 1.0 0.0 "/Game/Sounds/Attenuations/Footstep.Footstep" 0))
          (:then_1
            (bind _returnvalue_2 (Game|SpawnActorfromClass "/Game/Blueprints/Doors/BP_Key.BP_Key_C" (Math|Conversions|ToTransform(Vector) (Variables|Default|GetActorLocation)) "Undefined" 0 0))
            (Variables|/Game/Blueprints/Doors/BP_Key.BP_Key_C|SetDoorReference _returnvalue_2 (Variables|Default|GetDoorReference))))))))

(event EventTick
  (params (DeltaSeconds :type Float%20%28single-precision%29)))

(event EventBeginPlay)

(fn ConstructionScript)