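; AI controller for the 7OCLOCK AI character, which runs its behavior tree and caches the controlled pawn on BeginPlay.
; Perception updates start a delayed loop that counts Sightings past a threshold, adding a short grace period before contact with the player.
; When the loop completes, it writes the sensed state to the CanSeePlayer blackboard key if the actor is the main character, then resets the counter.
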(event OnTargetPerceptionUpdated(AIPerception)
  (params (Actor :type Actor%20Object%20Reference) (Stimulus :type AI%20Stimulus%20Structure))
  ;[1 1 1] Count sightings to give time before contact with player
  (Utilities|WhileLoopwithDelay (<= (Variables|Default|GetSightings) 5) 0.1
    (:LoopBody
      (bind _output_get (Variables|Default|SetSightings (+ (Variables|Default|GetSightings) 1)))
      (Development|PrintString (Utilities|String|Append (Utilities|String|ToString(Integer) _output_get) " Sightings") false))
    (:Completed
      ;[1 1 1] Set CanSeePlayer
      (Utilities|Casting|CastToBP_MainCharacter Actor)
      (AI|Components|Blackboard|SetValueasBool (AI|GetBlackboard 0) (Utilities|Name|MakeLiteralName "CanSeePlayer") (.bSuccessfullySensed (Utilities|Struct|BreakAIStimulus Stimulus)))
      (Variables|Default|SetSightings 0)
      (Development|PrintString "RESET" false true "(R=0.111672,G=1.000000,B=0.095488,A=1.000000)"))))

(event EventBeginPlay
  (AI|RunBehaviorTree "/Game/Blueprints/AI/BP_BT_7OCLOCK.BP_BT_7OCLOCK")
  (bind _asbp_ai_7oclock (Utilities|Casting|CastToBP_AI_7OCLOCK (Pawn|GetControlledPawn)))
  (Variables|Default|SetControlledPawn _asbp_ai_7oclock))

(fn ConstructionScript)