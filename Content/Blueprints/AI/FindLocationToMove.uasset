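; Behavior tree task that picks a random patrol destination for a BP_AI_7OCLOCK pawn.
; On execute it plays an audio message on the pawn, then selects a random actor from the pawn's CurrentPatrolPath.
; It writes a random navigable point near that actor to the BBLocation blackboard key and finishes successfully.
; A failed cast stops the graph without finishing the task.
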(event EventReceiveExecuteAI
  (params (OwnerController :type AI%20Controller%20Object%20Reference) (ControlledPawn :type Pawn%20Object%20Reference))
  (Class|BPiAudioManager|PlayAudio(Message) ControlledPawn)
  (Development|PrintString "Finding Random Location")
  (bind _asbp_ai_7oclock (Utilities|Casting|CastToBP_AI_7OCLOCK ControlledPawn))
  (AI|BehaviorTree|SetBlackboardValueasVector (Variables|Default|GetBB_Location) (.RandomLocation (Class|NavigationSystemV1|GetRandomPointinNavigableRadius (Transformation|GetActorLocation (Utilities|Array|Get(acopy) (Variables|/Game/Blueprints/AI/BP_AI_7OCLOCK.BP_AI_7OCLOCK_C|GetCurrentPatrolPath _asbp_ai_7oclock) (Math|Random|RandomInteger (Utilities|Array|Length (Variables|/Game/Blueprints/AI/BP_AI_7OCLOCK.BP_AI_7OCLOCK_C|GetCurrentPatrolPath _asbp_ai_7oclock))))) 1e+02 0 0)))
  (AI|BehaviorTree|FinishExecute true))