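; BP_AI_7OCLOCK is a monster AI that calls Dying on the player character when its capsule hits them, and drives its own audio.
; Tick toggles footstep audio by velocity, and a breathing sound starts on BeginPlay.
; PlayAudio switches on status: patrol plays grunts and fades out any chase audio, while chase stops breathing and triggers scream, chase sound and music.
; A DoOnce prevents repeated chase sounds until returning to patrol resets it and resumes breathing.
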(event OnComponentHit(CapsuleComponent)
  (params (HitComponent :type Primitive%20Component%20Object%20Reference) (OtherActor :type Actor%20Object%20Reference) (OtherComp :type Primitive%20Component%20Object%20Reference) (NormalImpulse :type Vector :default "0, 0, 0") (Hit :type Hit%20Result%20Structure%20%28by%20ref%29))
  (bind _returnvalue (Actor|GetActorOfClass "/Script/Bonhomme7Heure.MainCharacter"))
  (if (== OtherActor _returnvalue)
    (bind _asbp_main_character (Utilities|Casting|CastToBP_MainCharacter (Game|Player|GetPlayerPawn 0)))
    (Default|Dying _asbp_main_character)))

(event Custom|Resets%20Chasing%20Sounds
  (bind _returnvalue (Transformation|GetActorLocation))
  (Utilities|FlowControl|DoOnce false) ; enters at Reset
)

(event EventTick
  (params (DeltaSeconds :type Float%20%28single-precision%29))
  (bind _audiofootsteps (Variables|Default|GetAudioFootsteps))
  (if (> (Math|Vector|VectorLength (Transformation|GetVelocity self)) 1e+01)
    (Components|Activation|Activate _audiofootsteps false)
    (else
      (Components|Activation|Deactivate _audiofootsteps))))

(event EventPlayAudio
  (params (Status :type Byte :default 0))
  (bind _returnvalue (Transformation|GetActorLocation))
  (switch int (Math|Conversions|ToInteger(Byte) Status)
    (:0
      ;[1 1 1] Grunts on moving to new patrol location
      (Audio|SpawnSoundatLocation "/Game/Sounds/Cues/A_Monster_Grunts_Cue.A_Monster_Grunts_Cue" _returnvalue "0, 0, 0" 3.0 1.0 0.0 "/Game/Sounds/Attenuations/Footstep.Footstep" 0)
      (if (Utilities|IsValid (stale _returnvalue_2))
        ;[1 1 1] Back on patrol, music fades and back to normal breathing
        (Audio|Components|Audio|FadeOut (stale _returnvalue_3) 5.0 0.0 "Linear" :!class /Script/Engine.AudioComponent :!label _label)
        (Utilities|FlowControl|Sequence
          (:then_0
            (Audio|Components|Audio|Play (Variables|Default|GetBreath) 0.0))
          (:then_1
            (CallFunction|ResetsChasingSounds)))
        (elif (Utilities|IsValid (stale _returnvalue_3))
          (goto _label))))
    (:2
      (Audio|Components|Audio|Stop (Variables|Default|GetBreath))
      (Utilities|FlowControl|DoOnce false
        (:Completed
          ;[1 1 1] Monster Scream and start Chasing music
          (Audio|SpawnSoundatLocation "/Game/Sounds/Cues/A_Monster_Scream.A_Monster_Scream" _returnvalue "0, 0, 0" 3.0 1.0 0.0 "/Game/Sounds/Attenuations/Footstep.Footstep" 0)
          (bind _returnvalue_2 (Audio|SpawnSoundatLocation "/Game/Sounds/Cues/A_Monster_Chase.A_Monster_Chase" _returnvalue "0, 0, 0" 3.0 1.0 0.0 "/Game/Sounds/Attenuations/Footstep.Footstep" 0 false))
          (Utilities|FlowControl|Delay 0.5)
          (bind _returnvalue_3 (Audio|SpawnSound2D "/Game/Sounds/Cues/A_Music_Chasing_Cue.A_Music_Chasing_Cue" 1.0 1.0 0.0 0)))))))

(event EventBeginPlay
  (Audio|Components|Audio|Play (Variables|Default|GetBreath) 0.0))

(fn ConstructionScript)