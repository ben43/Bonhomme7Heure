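; BP_Lever is an interactable lever that triggers a referenced furnace and resets the player's movement on Interact.
; A Gate, opened and closed by Box overlap, guards only the sound and handle animation, not the furnace trigger.
; Two chained timelines lower then raise the handle by adding Alpha to its world Z each update.
; Actor overlap caches the BP_MainCharacter reference.
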(event OnComponentBeginOverlap(Box)
  (params (OverlappedComponent :type Primitive%20Component%20Object%20Reference) (OtherActor :type Actor%20Object%20Reference) (OtherComp :type Primitive%20Component%20Object%20Reference) (OtherBodyIndex :type Integer) (bFromSweep :type Boolean) (SweepResult :type Hit%20Result%20Structure%20%28by%20ref%29))
  (bind _sm_lever_handle (Variables|Default|GetSM_Lever_Handle))
  (bind _returnvalue (Transformation|GetWorldLocation _sm_lever_handle))
  (bind (_x _y _z) (Math|Vector|BreakVector _returnvalue))
  (Utilities|FlowControl|Gate true) ; enters at Open
)

(event OnComponentEndOverlap(Box)
  (params (OverlappedComponent :type Primitive%20Component%20Object%20Reference) (OtherActor :type Actor%20Object%20Reference) (OtherComp :type Primitive%20Component%20Object%20Reference) (OtherBodyIndex :type Integer))
  (bind _sm_lever_handle (Variables|Default|GetSM_Lever_Handle))
  (bind _returnvalue (Transformation|GetWorldLocation _sm_lever_handle))
  (bind (_x _y _z) (Math|Vector|BreakVector _returnvalue))
  (Utilities|FlowControl|Gate true) ; enters at Close
)

(event Custom|ReverseAnimation
  (bind _sm_lever_handle (Variables|Default|GetSM_Lever_Handle))
  (bind _returnvalue (Transformation|GetWorldLocation _sm_lever_handle))
  (bind (_x _y _z) (Math|Vector|BreakVector _returnvalue))
  (bind _alpha (Timeline|LeverUp PlayFromStart)
    (:Update
      (Transformation|SetWorldLocation (Variables|Default|GetSM_Lever_Handle) (Math|Vector|MakeVector _x _y (+ _z _alpha)) false false))))

(event EventBeginPlay)

(event Collision|EventActorBeginOverlap
  (params (OtherActor :type Actor%20Object%20Reference))
  (bind _returnvalue (Actor|GetActorOfClass "/Game/Blueprints/CharacterNMovement/BP_MainCharacter.BP_MainCharacter_C"))
  (Variables|Default|SetPlayerRef _returnvalue))

(event EventInteract
  (params (FromEnigma? :type Boolean))
  (bind _sm_lever_handle (Variables|Default|GetSM_Lever_Handle))
  (bind _returnvalue (Transformation|GetWorldLocation _sm_lever_handle))
  (bind (_x _y _z) (Math|Vector|BreakVector _returnvalue))
  (Default|Trigger (Variables|Default|GetFurnaceRef))
  (Default|ResetMovement (Variables|Default|GetPlayerRef))
  (Utilities|FlowControl|Gate true
    (:Exit
      (Audio|SpawnSoundatLocation "/Game/Sounds/SFX/Safe/A_SafeOpening.A_SafeOpening" _returnvalue "0, 0, 0" 1.0 1.0 0.0 0 0)
      (bind _alpha (Timeline|LeverDown PlayFromStart)
        (:Update
          (Transformation|SetWorldLocation (Variables|Default|GetSM_Lever_Handle) (Math|Vector|MakeVector _x _y (- _z _alpha)) false false))
        (:Finished
          (CallFunction|ReverseAnimation))))))

(fn ConstructionScript)