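; BP_Door is an interactable door that only the adult character can open.
; Its box overlap shows or removes a BP_WGT_Interact prompt and records whether an adult or child character is in range.
; On Interacted, an adult flip-flops the mesh between adding 90 degrees of yaw and negating its current yaw.
; A child instead gets the prompt replaced for two seconds by a "not an adult" notice, currently the same widget class.
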(event OnComponentBeginOverlap(Box)
  (params (OverlappedComponent :type Primitive%20Component%20Object%20Reference) (OtherActor :type Actor%20Object%20Reference) (OtherComp :type Primitive%20Component%20Object%20Reference) (OtherBodyIndex :type Integer) (bFromSweep :type Boolean) (SweepResult :type Hit%20Result%20Structure%20%28by%20ref%29))
  (Utilities|Casting|CastToBP_AdultCharacter OtherActor
    (:then
      (bind _returnvalue (UserInterface|CreateWidget "/Game/UI/BP_WGT_Interact.BP_WGT_Interact_C"))
      (bind _output_get (Variables|Default|SetInteractWidget _returnvalue))
      (UserInterface|Viewport|AddtoViewport _output_get 0)
      (Variables|Default|SetCharacterInRange true)
      (Variables|Default|SetAdultCharacter? true))
    (:CastFailed
      (Utilities|Casting|CastToBP_ChildCharacter OtherActor)
      (bind _returnvalue_2 (UserInterface|CreateWidget "/Game/UI/BP_WGT_Interact.BP_WGT_Interact_C"))
      (bind _output_get_2 (Variables|Default|SetInteractWidget _returnvalue_2))
      (UserInterface|Viewport|AddtoViewport _output_get_2 0)
      (Variables|Default|SetAdultCharacter? false)
      (Variables|Default|SetCharacterInRange true))))

(event OnComponentEndOverlap(Box)
  (params (OverlappedComponent :type Primitive%20Component%20Object%20Reference) (OtherActor :type Actor%20Object%20Reference) (OtherComp :type Primitive%20Component%20Object%20Reference) (OtherBodyIndex :type Integer))
  (bind _interactwidget (Variables|Default|GetInteractWidget))
  (Utilities|Casting|CastToBP_AdultCharacter OtherActor
    (:then
      (Widget|RemovefromParent _interactwidget)
      (Variables|Default|SetCharacterInRange false))
    (:CastFailed
      (Utilities|Casting|CastToBP_ChildCharacter OtherActor)
      (Widget|RemovefromParent _interactwidget)
      (Variables|Default|SetCharacterInRange false))))

(event Custom|Interacted
  (bind _staticmesh (Variables|Default|GetStaticMesh))
  (bind _returnvalue (Transformation|GetWorldRotation _staticmesh))
  (bind (_roll _pitch _yaw) (Math|Rotator|BreakRotator _returnvalue))
  (if (Variables|Default|GetCharacterInRange)
    (if (Variables|Default|GetAdultCharacter?)
      (Utilities|FlowControl|FlipFlop
        (:A
          (Transformation|SetWorldRotation _staticmesh (Math|Rotator|MakeRotator _roll _pitch (+ _yaw 9e+01)) false false))
        (:B
          (Transformation|SetWorldRotation _staticmesh (Math|Rotator|MakeRotator _roll _pitch (- 0.0 _yaw)) false false)))
      (else
        (Widget|RemovefromParent (Variables|Default|GetInteractWidget))
        ;[1 1 1] Create a not an adult widget
        (bind _returnvalue_2 (UserInterface|CreateWidget "/Game/UI/BP_WGT_Interact.BP_WGT_Interact_C"))
        (UserInterface|Viewport|AddtoViewport _returnvalue_2 0)
        (Utilities|FlowControl|Delay 2.0)
        (Widget|RemovefromParent _returnvalue_2)))))

(fn ConstructionScript)