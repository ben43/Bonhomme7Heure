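; BP_SimulatedActor is a configurable mesh actor that plays a collision sound on impacts, with mesh and mass override set in the construction script.
; Hits above a speed threshold spawn a plate collision cue at the mesh, with volume scaled by velocity and Footstep attenuation.
; A DoOnce gate limits repeats, resetting after a short delay only if the spawned sound reports it is playing.
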(event OnComponentBeginOverlap(StaticMesh)
  (params (OverlappedComponent :type Primitive%20Component%20Object%20Reference) (OtherActor :type Actor%20Object%20Reference) (OtherComp :type Primitive%20Component%20Object%20Reference) (OtherBodyIndex :type Integer) (bFromSweep :type Boolean) (SweepResult :type Hit%20Result%20Structure%20%28by%20ref%29)))

(event OnComponentHit(StaticMesh)
  (params (HitComponent :type Primitive%20Component%20Object%20Reference) (OtherActor :type Actor%20Object%20Reference) (OtherComp :type Primitive%20Component%20Object%20Reference) (NormalImpulse :type Vector :default "0, 0, 0") (Hit :type Hit%20Result%20Structure%20%28by%20ref%29))
  (bind _staticmesh (Variables|Default|GetStaticMesh))
  (bind _returnvalue (Transformation|GetComponentVelocity _staticmesh))
  (bind _returnvalue_2 (Math|Vector|VectorLength _returnvalue))
  (if (> _returnvalue_2 35.0)
    (Utilities|FlowControl|DoOnce false
      (:Completed
        (bind _returnvalue_3 (Audio|SpawnSoundatLocation "/Game/Sounds/Cues/A_Collision_Plates_Cue.A_Collision_Plates_Cue" (Transformation|GetWorldLocation (Variables|Default|GetStaticMesh)) "0, 0, 0" (Math|Float|MapRangeClamped _returnvalue_2 0.0 5e+02 0.0 8.0) 1.0 0.0 "/Game/Sounds/Attenuations/Footstep.Footstep" 0))
        (if (Audio|Components|Audio|IsPlaying _returnvalue_3)
          (Utilities|FlowControl|Delay 0.2)
          (CallFunction|ResetSound))))))

(event Custom|Reset%20Sound
  (Utilities|FlowControl|DoOnce false) ; enters at Reset
)

(event EventBeginPlay)

(event Collision|EventActorBeginOverlap
  (params (OtherActor :type Actor%20Object%20Reference)))

(fn ConstructionScript
  (bind _staticmesh (Variables|Default|GetStaticMesh))
  (Components|StaticMesh|SetStaticMesh _staticmesh (Variables|Default|GetMesh))
  (Class|PrimitiveComponent|SetMassOverrideinKg _staticmesh "None" (Variables|Default|GetMass) true))