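; Interactable actor with a configurable mesh that lets the player skip ahead to day in the day/night cycle.
; Its Box overlap shows a custom prompt widget and sets CloseEnough while a BP_ChildCharacter is inside, clearing both on exit.
; Interact resets BP_MainCharacter movement and prints a debug string regardless of range, then triggers CallGoToDay through GoToNextCycle only when CloseEnough is set.
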(event OnComponentBeginOverlap(Box)
  (params (OverlappedComponent :type Primitive%20Component%20Object%20Reference) (OtherActor :type Actor%20Object%20Reference) (OtherComp :type Primitive%20Component%20Object%20Reference) (OtherBodyIndex :type Integer) (bFromSweep :type Boolean) (SweepResult :type Hit%20Result%20Structure%20%28by%20ref%29))
  (CallFunction|DetectPlayerEntering OtherActor))

(event OnComponentEndOverlap(Box)
  (params (OverlappedComponent :type Primitive%20Component%20Object%20Reference) (OtherActor :type Actor%20Object%20Reference) (OtherComp :type Primitive%20Component%20Object%20Reference) (OtherBodyIndex :type Integer))
  (CallFunction|DetectPlayerLeaving OtherActor))

(event EventBeginPlay)

(event EventInteract
  (params (FromEnigma? :type Boolean))
  (bind _asbp_main_character (Utilities|Casting|CastToBP_MainCharacter (Game|GetPlayerCharacter 0)))
  (Default|ResetMovement _asbp_main_character)
  (Development|PrintString "Hello")
  (if (Variables|Default|GetCloseEnough)
    (CallFunction|GotoNextCycle)))

(fn ConstructionScript
  (Components|StaticMesh|SetStaticMesh (Variables|Default|GetStaticMesh) (Variables|Mesh|GetMesh)))

(fn GotoNextCycle
  (Default|CallGotoDay))

(fn DetectPlayerEntering
  (params (Object :type Object%20Object%20Reference))
  (Utilities|Casting|CastToBP_ChildCharacter Object)
  (bind _returnvalue (UserInterface|CreateWidget "/Game/UI/BP_WGT_CustomPrompt.BP_WGT_CustomPrompt_C" (Game|GetPlayerController 0)))
  (Variables|/Game/UI/BP_WGT_CustomPrompt.BP_WGT_CustomPrompt_C|SetTextToDisplay _returnvalue (Variables|Default|GetTextToDisplay))
  (bind _output_get (Variables|Default|SetPrompt_Widget _returnvalue))
  (UserInterface|Viewport|AddtoViewport _output_get 0)
  (Variables|Default|SetCloseEnough true))

(fn DetectPlayerLeaving
  (params (Actor :type Object%20Object%20Reference))
  (Utilities|Casting|CastToBP_ChildCharacter Actor)
  (Widget|RemovefromParent (Variables|Default|GetPrompt_Widget))
  (Variables|Default|SetCloseEnough false))