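; BP_GoToNight is an interaction point in the day/night skip feature that requests a switch to night.
; When a BP_AdultCharacter enters, DetectPlayerEntering shows a custom prompt widget and sets CloseEnough; DetectPlayerLeaving removes the prompt and clears the flag, both printing it.
; GoToNextCycle fires the GoToNight call, with no overlap or input triggers wired in this graph.
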(event EventBeginPlay
  (|CallParentFunction) ; This node is disabled and will not be called.\nDrag off pins to build functionality.
)

(event Collision|EventActorBeginOverlap
  (params (OtherActor :type Actor%20Object%20Reference)))

(event EventTick
  (params (DeltaSeconds :type Float%20%28single-precision%29)))

(fn ConstructionScript
  (|CallParentFunction))

(fn DetectPlayerEntering
  (params (Object :type Object%20Object%20Reference))
  (Utilities|Casting|CastToBP_AdultCharacter Object)
  (bind _returnvalue (UserInterface|CreateWidget "/Game/UI/BP_WGT_CustomPrompt.BP_WGT_CustomPrompt_C" (Game|GetPlayerController 0)))
  (Variables|/Game/UI/BP_WGT_CustomPrompt.BP_WGT_CustomPrompt_C|SetTextToDisplay _returnvalue (Variables|Default|GetTextToDisplay))
  (bind _output_get (Variables|Default|SetInteract_Prompt _returnvalue))
  (UserInterface|Viewport|AddtoViewport _output_get 0)
  (bind _output_get_2 (Variables|Default|SetCloseEnough true))
  (Development|PrintString (Utilities|String|ToString(Boolean) _output_get_2)))

(fn DetectPlayerLeaving
  (params (Actor :type Object%20Object%20Reference))
  (Utilities|Casting|CastToBP_AdultCharacter Actor)
  (Widget|RemovefromParent (Variables|Default|GetInteract_Prompt))
  (bind _output_get (Variables|Default|SetCloseEnough false))
  (Development|PrintString (Utilities|String|ToString(Boolean) _output_get)))

(fn GotoNextCycle
  (Default|CallGotoNight))