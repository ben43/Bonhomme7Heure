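; Adult character Blueprint that plays a voice line for the first enigma when it begins play.
; On BeginPlay it finds BP_ProgressionManager and acts only when the EnigmaFinished value is zero.
; The manager's 1stSentenceSaid flag makes the dad's intro line play once, with later spawns playing a louder random line from a pool.
; Tick and overlap events are disabled.
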(event EventBeginPlay
  (|CallParentFunction)
  (bind _returnvalue (Actor|GetActorOfClass "/Game/Blueprints/BP_ProgressionManager.BP_ProgressionManager_C"))
  (switch int (Variables|/Game/Blueprints/BP_ProgressionManager.BP_ProgressionManager_C|GetEnigmaFinished _returnvalue)
    (:0
      (if (Variables|/Game/Blueprints/BP_ProgressionManager.BP_ProgressionManager_C|Get1stSentenceSaid _returnvalue)
        (Audio|PlaySound2D (Utilities|Array|Get(acopy) (Variables|Default|GetRandomVoiceLineEnigma1) (Math|Random|RandomInteger 2)) 2.0 1.0 0.0 0 0)
        (else
          (Variables|/Game/Blueprints/BP_ProgressionManager.BP_ProgressionManager_C|Set1stSentenceSaid _returnvalue true)
          (Audio|PlaySound2D "/Game/Sounds/Voices/Dad/Dad1stEnigma.Dad1stEnigma" 1.0 1.0 0.0 0 0))))))

(event Collision|EventActorBeginOverlap
  (params (OtherActor :type Actor%20Object%20Reference)))

(event EventTick
  (params (DeltaSeconds :type Float%20%28single-precision%29))
  (|CallParentFunction DeltaSeconds) ; This node is disabled and will not be called.\nDrag off pins to build functionality.
)

(fn ConstructionScript
  (|CallParentFunction))