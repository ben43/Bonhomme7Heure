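; Child player character Blueprint that plays an opening voice line over ducked music when play begins.
; On BeginPlay it runs the parent logic, grants matches and switches on the progression manager's EnigmaFinished value.
; The default branch lowers the music class through a sound mix override and plays a random Enigma 1 voice line.
; When that audio finishes, a bound event fades the music back up.
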(event Custom|OnAudioFinished_Event_LiftMusic
  (Audio|SetSoundMixClassOverride "/Game/Sounds/SoundsClasses/B7H_SCM_Master.B7H_SCM_Master" "/Game/Sounds/SoundsClasses/B7H_Music.B7H_Music" 1.0 1.0 (Variables|Default|GetFadetime) true))

(event EventBeginPlay
  (|CallParentFunction)
  (Variables|Default|SetHasMatches? true)
  (bind _returnvalue (Actor|GetActorOfClass "/Game/Blueprints/BP_ProgressionManager.BP_ProgressionManager_C"))
  (switch int (Variables|/Game/Blueprints/BP_ProgressionManager.BP_ProgressionManager_C|GetEnigmaFinished _returnvalue)
    (:Default
      (Audio|SetSoundMixClassOverride "/Game/Sounds/SoundsClasses/B7H_SCM_Master.B7H_SCM_Master" "/Game/Sounds/SoundsClasses/B7H_Music.B7H_Music" 0.3 1.0 (Variables|Default|GetFadetime) true)
      (bind _returnvalue_2 (Audio|CreateSound2D (Utilities|Array|Get(acopy) (Variables|Default|GetEnigma1RandomVoiceLine) (Math|Random|RandomInteger 2)) 1.0 1.0 0.0 0))
      (Audio|Components|Audio|Play _returnvalue_2 0.0)
      (EventDispatchers|AssignOnAudioFinished _returnvalue_2 (delegate Custom|OnAudioFinished_Event_LiftMusic)))))

(event Collision|EventActorBeginOverlap
  (params (OtherActor :type Actor%20Object%20Reference)))

(event EventTick
  (params (DeltaSeconds :type Float%20%28single-precision%29))
  (|CallParentFunction DeltaSeconds) ; This node is disabled and will not be called.\nDrag off pins to build functionality.
)

(fn ConstructionScript
  (|CallParentFunction))