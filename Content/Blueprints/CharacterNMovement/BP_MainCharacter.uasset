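; Main player character, handling movement, sprint stamina, crouch, footstep audio, interaction, pause and death screens.
; Tick updates stamina, a match-gated lighter's intensity and speed-scaled camera shake.
; Delayed loops change madness in madness or sanity zones, driving a dynamic post-effect material and audio volume.
; Camera traces send BPi_Interact messages, C++ Grabber slows walking for simulated actors, and a spawned ModelViewer displays meshes with UI-only input.
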(event Custom|GainMadness
  ;[1 1 1] MadnessManager
  (Utilities|WhileLoopwithDelay (Variables|Default|GetInMadnessZone) 0.01
    (:LoopBody
      (if (not (== (Variables|Default|GetMadnessLevel) 1.0))
        (bind _output_get (Variables|Default|SetMadnessLevel (Math|Float|Clamp(Float) (+ (Variables|Default|GetMadnessLevel) 0.0015))))
        (Rendering|Material|SetScalarParameterValue (stale EventBeginPlay _returnvalue) "MadnessControl" _output_get :!class /Script/Engine.MaterialInstanceDynamic)
        (Audio|Components|Audio|SetVolumeMultiplier (Variables|Default|GetAudioMadness) (Math|Float|Power _output_get 2.0) :!class /Script/Engine.AudioComponent)))))

(event Custom|LoseMadness
  ;[1 1 1] MadnessManager
  (Utilities|WhileLoopwithDelay (Variables|Default|GetInSanityGainingZone) 0.1
    (:LoopBody
      (if (not (<= (Variables|Default|GetMadnessLevel) 0.0))
        (bind _output_get (Variables|Default|SetMadnessLevel (Math|Float|Clamp(Float) (- (Variables|Default|GetMadnessLevel) 0.005))))
        (Rendering|Material|SetScalarParameterValue (stale EventBeginPlay _returnvalue) "MadnessControl" _output_get :!class /Script/Engine.MaterialInstanceDynamic)
        (Audio|Components|Audio|SetVolumeMultiplier (Variables|Default|GetAudioMadness) _output_get :!class /Script/Engine.AudioComponent)))))

(event Custom|Dying
  (bind _returnvalue (Game|GetPlayerController 0))
  ;[1 1 1] Dying
  (Utilities|FlowControl|DoOnce false
    (:Completed
      (Game|SetGamePaused true)
      (Input|SetInputModeUIOnly _returnvalue 0 "DoNotLock")
      (Variables|/Script/Engine.PlayerController|SetbShowMouseCursor _returnvalue true)
      (bind _returnvalue_2 (UserInterface|CreateWidget "/Game/UI/BP_WGT_Dead.BP_WGT_Dead_C" _returnvalue))
      (UserInterface|Viewport|AddtoViewport _returnvalue_2 0))))

(event Custom|3DObjectViewer
  (params (MeshToSpawn :type Static%20Mesh%20Object%20Reference))
  (bind _returnvalue (Game|GetPlayerController 0))
  (bind _charactermovement (Variables|Character|GetCharacterMovement))
  (bind _charactermovement_2 (Variables|Character|GetCharacterMovement))
  ;[1 1 1] ObjectViewer
  (Components|Movement|StopMovementImmediately _charactermovement_2)
  (Class|NavMovementComponent|StopActiveMovement _charactermovement_2)
  (bind _returnvalue_2 (Game|SpawnActorfromClass "/Game/Blueprints/ModelViewer.ModelViewer_C" (Transformation|GetWorldTransform (Variables|Default|GetModelViewerPosition)) "Undefined" 0 0))
  (Default|SetStaticMesh _returnvalue_2 MeshToSpawn)
  (Input|SetInputModeUIOnly _returnvalue 0 "DoNotLock")
  (Components|Movement|StopMovementImmediately _charactermovement)
  (Class|NavMovementComponent|StopActiveMovement _charactermovement)
  (Variables|/Script/Engine.PlayerController|SetbShowMouseCursor _returnvalue true)
  (Rendering|SetVisibility (Variables|Default|GetUI) true false))

(event Custom|ObjectViewerDestrution
  (bind _returnvalue (Game|GetPlayerController 0))
  (Default|Destruction (stale Custom|3DObjectViewer _returnvalue_2))
  (Input|SetInputModeGameOnly _returnvalue)
  (Variables|/Script/Engine.PlayerController|SetbShowMouseCursor _returnvalue false)
  (Rendering|SetVisibility (Variables|Default|GetUI) false false))

(event EventBeginPlay
  ;[1 1 1] BeginPlay
  (Utilities|FlowControl|Sequence
    (:then_1
      (bind _returnvalue (Rendering|Material|CreateDynamicMaterialInstance (Variables|Default|GetMadness) 0 "/Game/Materials/Instances/MI_MadnessFX.MI_MadnessFX" "None" :!class /Script/Engine.PrimitiveComponent))
      (Rendering|Material|SetScalarParameterValue _returnvalue "MadnessControl" 0.0 :!class /Script/Engine.MaterialInstanceDynamic))))

(event EventTick
  (params (DeltaSeconds :type Float%20%28single-precision%29))
  (bind _returnvalue (Game|GetPlayerCameraManager 0))
  (bind _self self)
  (bind _lighter (Variables|Default|GetLighter))
  (bind _returnvalue_2 (Transformation|GetVelocity _self))
  (bind _returnvalue_3 (Math|Vector|VectorLength _returnvalue_2))
  ;[1 1 1] StaminaManager
  (Utilities|FlowControl|Sequence
    (:then_0
      (if (Variables|Stamina|GetRegenStamina)
        (Variables|Stamina|SetStamina (Math|Float|Clamp(Float) (+ (Variables|Stamina|GetStamina) (Variables|Stamina|GetStaminaGainRate)) 0.0 1e+02))
        (else
          (Variables|Stamina|SetStamina (Math|Float|Clamp(Float) (- (Variables|Stamina|GetStamina) (Variables|Stamina|GetStaminaLossRate)) 0.0 1e+02)))))
    (:then_1
      (if (<= (Variables|Stamina|GetStamina) 0.0)
        (Variables|/Script/Engine.CharacterMovementComponent|SetMaxWalkSpeed (Variables|Character|GetCharacterMovement) (Variables|MovementSpeed|GetMaxWalkSpeed))))
    (:then_2
      ;[1 1 1] Matches
      (if (stale Input|ActionEvents|InputActionFlashlight _output_get)
        (Utilities|FlowControl|Sequence
          (:then_0
            (bind _output_get (Variables|Light|SetLighterIntensity (Math|Float|Clamp(Float) (+ (Variables|Light|GetLighterIntensity) 5e+02) 0.0 3e+03)))
            (Rendering|Components|Light|SetIntensity _lighter _output_get)
            (if (> (Variables|Light|GetLighterIntensity) (Variables|Default|GetLighterMaxIntensity))
              (Rendering|Components|Light|SetIntensity _lighter (stale _output_get_2) :!label _label)))
          (:then_1
            ;;[0.5117 0.9099 1] Audio
            (Utilities|FlowControl|DoOnce false :!label _label_2
              (:Completed
                (Audio|SpawnSoundAttached "/Game/Sounds/Cues/A_LighterIgnite_Cue.A_LighterIgnite_Cue" (Variables|Default|GetFollowCamera) "None" "0, 0, 0" "0, 0, 0" "KeepRelativeOffset" false 3.0 1.0 0.0 "/Game/Sounds/Attenuations/Footstep.Footstep" 0)
                (Utilities|FlowControl|Delay 3.0)
                (goto _label_2 Reset)))))
        (else
          (bind _output_get_2 (Variables|Light|SetLighterIntensity (Math|Float|Clamp(Float) (- (Variables|Light|GetLighterIntensity) 1e+01) 0.0 3e+03)))
          (goto _label))))
    (:then_3
      ;[1 1 1] CameraShakes
      (if (> _returnvalue_3 0.0)
        (bind _returnvalue_4 (Class|PlayerCameraManager|PlayCameraShake _returnvalue "/Game/Blueprints/CharacterNMovement/BP_CameraShake_Running.BP_CameraShake_Running_C" (/ _returnvalue_3 1.5e+02) "CameraLocal" "0, 0, 0"))
        (else
          (CameraShakes|StopCameraShake _returnvalue _returnvalue_4 false))))))

(event EventAddMatches
  ;[1 1 1] Matches
  (Variables|Default|SetHasMatches? true))

(event Input|ActionEvents|InputActionFlashlight
  (params (Key :type Key%20Structure :default "None"))
  (bind _lighter (Variables|Default|GetLighter))
  ;[1 1 1] Matches
  (:Pressed
    (if (Variables|Default|GetHasMatches?)
      (if (<= (Variables|Light|GetLighterIntensity) 0.0)
        (bind _output_get (Variables|Default|SetLighterOn? true))
        (if _output_get
          (Utilities|FlowControl|Sequence
            (:then_0
              (bind _output_get_2 (Variables|Light|SetLighterIntensity (Math|Float|Clamp(Float) (+ (Variables|Light|GetLighterIntensity) 5e+02) 0.0 3e+03)))
              (Rendering|Components|Light|SetIntensity _lighter _output_get_2)
              (if (> (Variables|Light|GetLighterIntensity) (Variables|Default|GetLighterMaxIntensity))
                (Rendering|Components|Light|SetIntensity _lighter (stale _output_get_3) :!label _label)))
            (:then_1
              ;;[0.5117 0.9099 1] Audio
              (Utilities|FlowControl|DoOnce false :!label _label_2
                (:Completed
                  (Audio|SpawnSoundAttached "/Game/Sounds/Cues/A_LighterIgnite_Cue.A_LighterIgnite_Cue" (Variables|Default|GetFollowCamera) "None" "0, 0, 0" "0, 0, 0" "KeepRelativeOffset" false 3.0 1.0 0.0 "/Game/Sounds/Attenuations/Footstep.Footstep" 0)
                  (Utilities|FlowControl|Delay 3.0)
                  (goto _label_2 Reset)))))
          (else
            (bind _output_get_3 (Variables|Light|SetLighterIntensity (Math|Float|Clamp(Float) (- (Variables|Light|GetLighterIntensity) 1e+01) 0.0 3e+03)))
            (goto _label))))))
  (:Released
    (Variables|Default|SetLighterOn? false)))

(event Input|ActionEvents|InputActionGrabInput
  (params (Key :type Key%20Structure :default "None"))
  (bind _charactermovement (Variables|Character|GetCharacterMovement))
  (bind _grabber (Variables|Default|GetGrabber))
  (bind _actorshits (Variables|/Script/Bonhomme7Heure.Grabber|GetActorsHits _grabber))
  (bind _returnvalue (Utilities|GetClass _actorshits))
  (bind _returnvalue_2 (Utilities|ClassIsChildOf _returnvalue "/Game/Blueprints/EnigmaBP/BP_SimulatedActor.BP_SimulatedActor_C"))
  ;[1 1 1] InteractionDetector
  ;;[1 1 1] Call the Grabber from Grabber.cpp
  (:Pressed
    (Class|Grabber|Grab _grabber)
    (if _returnvalue_2
      ;[1 1 1] Slowdown Player when objects are grabbed
      (Variables|Default|SetIsGrabable? _returnvalue_2)
      (Variables|Default|SetInitialMaxWalkSpeed (Variables|/Script/Engine.CharacterMovementComponent|GetMaxWalkSpeed _charactermovement))
      (Variables|/Script/Engine.CharacterMovementComponent|SetMaxWalkSpeed _charactermovement (Variables|Default|GetSlowdownAmount))))
  (:Released
    (Class|Grabber|Release _grabber)
    (if (Variables|Default|GetIsGrabable?)
      (Variables|/Script/Engine.CharacterMovementComponent|SetMaxWalkSpeed _charactermovement (Variables|Default|GetInitialMaxWalkSpeed)))))

(event Input|ActionEvents|InputActionJump
  (params (Key :type Key%20Structure :default "None"))
  ;[1 1 1] Movement
  ;;[1 1 1] Call Movement from .cpp file
  (:Pressed
    (Character|Jump))
  (:Released
    (Character|StopJumping)))

(event Input|ActionEvents|InputActionPauseButton
  (params (Key :type Key%20Structure :default "None"))
  (bind _returnvalue (Game|GetPlayerController 0))
  ;[1 1 1] Pause
  (:Pressed
    (bind _returnvalue_2 (UserInterface|CreateWidget "/Game/UI/BP_WGT_PauseMenu.BP_WGT_PauseMenu_C" _returnvalue))
    (UserInterface|Viewport|AddtoViewport _returnvalue_2 0)
    (Input|SetInputModeGameOnly _returnvalue)
    (Variables|/Script/Engine.PlayerController|SetbShowMouseCursor _returnvalue true)
    (Game|SetGamePaused true)))

(event Input|ActionEvents|InputActionCrouch
  (params (Key :type Key%20Structure :default "None"))
  (bind _returnvalue (Game|GetPlayerCharacter 0))
  ;[1 1 1] Movement
  ;;[1 1 1] Crouch
  (:Pressed
    (Utilities|FlowControl|FlipFlop
      (:A
        (Character|Crouch _returnvalue))
      (:B
        (Character|UnCrouch _returnvalue)))))

(event Input|ActionEvents|InputActionInteract_Button
  (params (Key :type Key%20Structure :default "None"))
  (bind _followcamera (Variables|Default|GetFollowCamera))
  (bind _returnvalue (Transformation|GetWorldLocation _followcamera))
  ;[1 1 1] InteractionDetector
  (:Pressed
    (bind (_outhit _returnvalue_2) (Collision|LineTraceByChannel _returnvalue (+ _returnvalue (* (Math|Vector|GetForwardVector _followcamera) (Variables|Default|GetReach))) "TraceTypeQuery1" false 0 "None"))
    (if _returnvalue_2
      (if (Utilities|DoesObjectImplementInterface (.HitActor (Collision|BreakHitResult _outhit)) "/Game/Blueprints/BPi_Interact.BPi_Interact_C")
        (Class|BPiInteract|Interact(Message) (.HitActor (Collision|BreakHitResult _outhit)) false)))))

(event Input|ActionEvents|InputActionSprint
  (params (Key :type Key%20Structure :default "None"))
  (bind _charactermovement (Variables|Character|GetCharacterMovement))
  ;[1 1 1] Movement
  ;;[1 1 1] Sprinting
  (:Pressed
    (if (> (Variables|Stamina|GetStamina) 3e+01)
      (Variables|/Script/Engine.CharacterMovementComponent|SetMaxWalkSpeed _charactermovement (Variables|MovementSpeed|GetSprintSpeed))
      (Variables|Stamina|SetRegenStamina false)
      (else
        (Variables|/Script/Engine.CharacterMovementComponent|SetMaxWalkSpeed _charactermovement (Variables|MovementSpeed|GetMaxWalkSpeed) :!label _label)
        (Variables|Stamina|SetRegenStamina true))))
  (:Released
    (goto _label)))

(event Input|AxisEvents|InputAxisTurnCamera
  (params (AxisValue :type Float%20%28single-precision%29))
  ;[1 1 1] Movement
  ;;[1 1 1] Call Movement from .cpp file
  (Pawn|Input|AddControllerYawInput AxisValue))

(event Input|AxisEvents|InputAxisMoveForward
  (params (AxisValue :type Float%20%28single-precision%29))
  ;[1 1 1] Movement
  ;;[1 1 1] Call Movement from .cpp file
  (Class|MainCharacter|MoveForward AxisValue))

(event Input|AxisEvents|InputAxisMoveRight
  (params (AxisValue :type Float%20%28single-precision%29))
  ;[1 1 1] Movement
  ;;[1 1 1] Call Movement from .cpp file
  (Class|MainCharacter|MoveRight AxisValue))

(event Input|AxisEvents|InputAxisLookUpCamera
  (params (AxisValue :type Float%20%28single-precision%29))
  ;[1 1 1] Movement
  ;;[1 1 1] Call Movement from .cpp file
  (Pawn|Input|AddControllerPitchInput AxisValue))

(event Input|KeyboardEvents|W
  (params (Key :type Key%20Structure :default "None"))
  (bind _audiofootstep (Variables|Default|GetAudioFootstep))
  ;[1 1 1] Movement
  ;;[0.5117 0.9099 1] Player Footsteps Audio
  (:Pressed
    (Components|Activation|Activate _audiofootstep false))
  (:Released
    (Components|Activation|Deactivate _audiofootstep)))

(event Input|KeyboardEvents|D
  (params (Key :type Key%20Structure :default "None"))
  (bind _audiofootstep (Variables|Default|GetAudioFootstep))
  ;[1 1 1] Movement
  ;;[0.5117 0.9099 1] Player Footsteps Audio
  (:Pressed
    (Components|Activation|Activate _audiofootstep false))
  (:Released
    (Components|Activation|Deactivate _audiofootstep)))

(event Input|KeyboardEvents|A
  (params (Key :type Key%20Structure :default "None"))
  (bind _audiofootstep (Variables|Default|GetAudioFootstep))
  ;[1 1 1] Movement
  ;;[0.5117 0.9099 1] Player Footsteps Audio
  (:Pressed
    (Components|Activation|Activate _audiofootstep false))
  (:Released
    (Components|Activation|Deactivate _audiofootstep)))

(event Input|KeyboardEvents|S
  (params (Key :type Key%20Structure :default "None"))
  (bind _audiofootstep (Variables|Default|GetAudioFootstep))
  ;[1 1 1] Movement
  ;;[0.5117 0.9099 1] Player Footsteps Audio
  (:Pressed
    (Components|Activation|Activate _audiofootstep false))
  (:Released
    (Components|Activation|Deactivate _audiofootstep)))

(fn ConstructionScript
  (bind _lighter (Variables|Default|GetLighter))
  (Class|LightComponent|SetTemperature _lighter (Variables|Light|GetLighterTemperature))
  (Rendering|Components|Light|SetIntensity _lighter (Variables|Light|GetLighterIntensity)))

(fn ActorHit)

(fn SlowdownWalk
  (params (NewMaxWalkSpeed :type Float%20%28single-precision%29)))

(fn Interact
  (params (FromEnigma? :type Boolean))
  (return))