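; BP_Teddy is an interactable teddy that gradually lowers the main character's madness level.
; A Box overlap stores the player, shows an interact widget and enables interaction, while leaving removes the widget and disables it.
; PlayerInteract starts a delayed loop that steps MadnessLevel down and prints it, ending when the player leaves or madness reaches zero.
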(event OnComponentBeginOverlap(Box)
  (params (OverlappedComponent :type Primitive%20Component%20Object%20Reference) (OtherActor :type Actor%20Object%20Reference) (OtherComp :type Primitive%20Component%20Object%20Reference) (OtherBodyIndex :type Integer) (bFromSweep :type Boolean) (SweepResult :type Hit%20Result%20Structure%20%28by%20ref%29))
  (bind _asbp_main_character (Utilities|Casting|CastToBP_MainCharacter OtherActor))
  (Variables|Default|SetPlayerReference _asbp_main_character)
  (bind _returnvalue (UserInterface|CreateWidget "/Game/UI/BP_WGT_Interact.BP_WGT_Interact_C" (Game|GetPlayerController 0)))
  (bind _output_get (Variables|Default|SetInteractWidget _returnvalue))
  (UserInterface|Viewport|AddtoViewport _output_get 0)
  (Variables|Default|SetCanInteract true))

(event OnComponentEndOverlap(Box)
  (params (OverlappedComponent :type Primitive%20Component%20Object%20Reference) (OtherActor :type Actor%20Object%20Reference) (OtherComp :type Primitive%20Component%20Object%20Reference) (OtherBodyIndex :type Integer))
  (Utilities|Casting|CastToBP_MainCharacter OtherActor)
  (Widget|RemovefromParent (Variables|Default|GetInteractWidget))
  (Variables|Default|SetCanInteract false))

(event Custom|PlayerInteract
  (bind _playerreference (Variables|Default|GetPlayerReference))
  (if (Variables|Default|GetCanInteract)
    (Utilities|WhileLoopwithDelay (Variables|Default|GetCanInteract) 0.2
      (:LoopBody
        (if (!= (Variables|/Game/Blueprints/BP_MainCharacter.BP_MainCharacter_C|GetMadnessLevel _playerreference) 0.0)
          (bind _output_get (Variables|/Game/Blueprints/BP_MainCharacter.BP_MainCharacter_C|SetMadnessLevel _playerreference (- (Variables|/Game/Blueprints/BP_MainCharacter.BP_MainCharacter_C|GetMadnessLevel _playerreference) 1.0)))
          (Development|PrintString (Utilities|String|ToString(Float) _output_get))
          (else
            ;[1 1 1] This is so the loop stop to save performances
            (Variables|Default|SetCanInteract false)))))))

(fn ConstructionScript)