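; Configurable trigger actor that fires ambient events when BP_MainCharacter overlaps its Box.
; Booleans select any mix of timed audio playback, moving between two locations, hiding or toggling the mesh, and switching or flickering a spot or point light.
; FlipFlops alternate states across overlaps.
; Flicker nests delayed loops with random intervals, running either a set count or endlessly.
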(event OnComponentBeginOverlap(Box)
  (params (OverlappedComponent :type Primitive%20Component%20Object%20Reference) (OtherActor :type Actor%20Object%20Reference) (OtherComp :type Primitive%20Component%20Object%20Reference) (OtherBodyIndex :type Integer) (bFromSweep :type Boolean) (SweepResult :type Hit%20Result%20Structure%20%28by%20ref%29))
  (bind _spotlight (Variables|Default|GetSpotLight))
  (bind _pointlight (Variables|Default|GetPointLight))
  (bind _pointlight_2 (Variables|Default|GetPointLight))
  (bind _spotlight_2 (Variables|Default|GetSpotLight))
  (bind _pointlight_3 (Variables|Default|GetPointLight))
  (bind _spotlight_3 (Variables|Default|GetSpotLight))
  (bind _objectlocations (Variables|MoveObject|GetObjectLocations))
  (Utilities|Casting|CastToBP_MainCharacter OtherActor)
  (Utilities|FlowControl|Sequence
    (:then_0
      ;[1 1 1] SoundPlayed
      (if (Variables|Sound|GetSound?)
        (if (Variables|Sound|GetRepeat)
          (Audio|Components|Audio|Play (Variables|Default|GetAudio) 0.0)
          (Variables|Sound|SetSound? false)
          (Utilities|FlowControl|Delay (Variables|Sound|GetSoundDuration))
          (Variables|Sound|SetSound? true)
          (if (Variables|Sound|Get1TimeSound)
            (Variables|Sound|SetRepeat false)))))
    (:then_1
      ;[1 1 1] ObjectMove
      (if (Variables|MoveObject|GetObjectMove?)
        (Utilities|FlowControl|FlipFlop
          (:A
            (Transformation|SetActorLocation (Utilities|Array|Get(acopy) _objectlocations 1) false false))
          (:B
            (Transformation|SetActorLocation (Utilities|Array|Get(acopy) _objectlocations) false false)))))
    (:then_2
      ;[1 1 1] Object Disappear
      (if (Variables|ObjectDisapearrance|GetObjectDisapear?)
        (if (Variables|ObjectDisapearrance|GetObjectWillReappear?)
          (Utilities|FlowControl|FlipFlop
            (:A
              (Rendering|SetVisibility (Variables|Default|GetStaticMesh) false false))
            (:B
              (Rendering|SetVisibility (Variables|Default|GetStaticMesh) true false)))
          (else
            (Rendering|SetVisibility (Variables|Default|GetStaticMesh) false false)))))
    (:then_3
      ;[1 1 1] LightOnAndOff
      (if (Variables|LightOnAndOff|GetLight?)
        (if (Variables|LightOnAndOff|GetSpotLight?)
          (if (Variables|LightOnAndOff|Get1Time?)
            (Rendering|SetVisibility _spotlight false false)
            (else
              (Utilities|FlowControl|FlipFlop
                (:A
                  (Rendering|SetVisibility _spotlight false false))
                (:B
                  (Rendering|SetVisibility _spotlight true false)))))
          (elif (Variables|LightOnAndOff|Get1Time?)
            (Rendering|SetVisibility _pointlight false false)
            (else
              (Utilities|FlowControl|FlipFlop
                (:A
                  (Rendering|SetVisibility _pointlight false false))
                (:B
                  (Rendering|SetVisibility _pointlight true false))))))))
    (:then_4
      ;[1 1 1] Light Flickering
      (if (Variables|LightFlickering|GetLightFlickering?)
        (if (Variables|LightFlickering|GetSpotlight?Flicker)
          (if (Variables|LightFlickering|GetLimitAmountOfFlicker)
            (Utilities|ForLoopwithDelay 0 (- (Variables|LightFlickering|GetNumberOfFlickering) 1) (Math|Random|RandomFloatinRange (Variables|LightFlickering|GetMinimumTimeFlicker) (Variables|LightFlickering|GetMaximumTimeFlicker))
              (:LoopBody
                (Utilities|ForLoopwithDelay 0 1 (Variables|LightFlickering|GetTimeOfTheFlickering)
                  (:LoopBody
                    (Utilities|FlowControl|FlipFlop
                      (:A
                        (Rendering|SetVisibility _spotlight_3 false false))
                      (:B
                        (Rendering|SetVisibility _spotlight_3 true false)))))))
            (else
              (Utilities|WhileLoopwithDelay true (Math|Random|RandomFloatinRange (Variables|LightFlickering|GetMinimumTimeFlicker) (Variables|LightFlickering|GetMaximumTimeFlicker))
                (:LoopBody
                  (Utilities|ForLoopwithDelay 0 1 (Variables|LightFlickering|GetTimeOfTheFlickering)
                    (:LoopBody
                      (Utilities|FlowControl|FlipFlop
                        (:A
                          (Rendering|SetVisibility _spotlight_2 false false))
                        (:B
                          (Rendering|SetVisibility _spotlight_2 true false)))))))))
          (elif (Variables|LightFlickering|GetLimitAmountOfFlicker)
            (Utilities|ForLoopwithDelay 0 (- (Variables|LightFlickering|GetNumberOfFlickering) 1) (Math|Random|RandomFloatinRange (Variables|LightFlickering|GetMinimumTimeFlicker) (Variables|LightFlickering|GetMaximumTimeFlicker))
              (:LoopBody
                (Utilities|ForLoopwithDelay 0 1 (Variables|LightFlickering|GetTimeOfTheFlickering)
                  (:LoopBody
                    (Utilities|FlowControl|FlipFlop
                      (:A
                        (Rendering|SetVisibility _pointlight_3 false false))
                      (:B
                        (Rendering|SetVisibility _pointlight_3 true false)))))))
            (else
              (Utilities|WhileLoopwithDelay true (Math|Random|RandomFloatinRange (Variables|LightFlickering|GetMinimumTimeFlicker) (Variables|LightFlickering|GetMaximumTimeFlicker))
                (:LoopBody
                  (Utilities|ForLoopwithDelay 0 1 (Variables|LightFlickering|GetTimeOfTheFlickering)
                    (:LoopBody
                      (Utilities|FlowControl|FlipFlop
                        (:A
                          (Rendering|SetVisibility _pointlight_2 false false))
                        (:B
                          (Rendering|SetVisibility _pointlight_2 true false))))))))))))))

(fn ConstructionScript)