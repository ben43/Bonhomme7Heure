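; An audio Blueprint that plays wind howl sounds at random positions inside a box volume.
; A looping timer started on BeginPlay fires every few seconds and spawns the cue at a random point within the box's scaled extents, with boosted volume and Footstep attenuation.
; Box overlap events toggle an InVolume flag, but the spawn logic never checks it, so sounds play regardless of overlap.
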(event OnComponentBeginOverlap(Box)
  (params (OverlappedComponent :type Primitive%20Component%20Object%20Reference) (OtherActor :type Actor%20Object%20Reference) (OtherComp :type Primitive%20Component%20Object%20Reference) (OtherBodyIndex :type Integer) (bFromSweep :type Boolean) (SweepResult :type Hit%20Result%20Structure%20%28by%20ref%29))
  (Variables|Default|SetInVolume? true))

(event OnComponentEndOverlap(Box)
  (params (OverlappedComponent :type Primitive%20Component%20Object%20Reference) (OtherActor :type Actor%20Object%20Reference) (OtherComp :type Primitive%20Component%20Object%20Reference) (OtherBodyIndex :type Integer))
  (Variables|Default|SetInVolume? false))

(event Custom|CallSpawnSound
  (bind _box (Variables|Default|GetBox))
  ;[1 1 1] Spawn a sound at random location in box
  (Audio|SpawnSoundatLocation "/Game/Sounds/Cues/A_WindHowls_Cue.A_WindHowls_Cue" (Math|Random|RandomPointinBoundingBox (Transformation|GetWorldLocation _box) (Components|Box|GetScaledBoxExtent _box)) "0, 0, 0" 5.0 1.0 0.0 "/Game/Sounds/Attenuations/Footstep.Footstep" 0))

(event EventBeginPlay
  ;[1 1 1] Spawn a sound at random location in box
  (Utilities|Time|SetTimerbyEvent (delegate Custom|CallSpawnSound) 4.0 true))

(fn ConstructionScript)