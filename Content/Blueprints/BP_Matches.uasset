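; BP_Matches is a matches pickup that the player character can interact with.
; A Box trigger creates and shows an interact prompt widget while BP_MainCharacter overlaps it, and removes it when the overlap ends.
; Interact shows the matches message on the character, plays a spatial pickup sound and a 2D success sound, resets the character's movement, then destroys the actor.
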(event OnComponentBeginOverlap(Box)
  (params (OverlappedComponent :type Primitive%20Component%20Object%20Reference) (OtherActor :type Actor%20Object%20Reference) (OtherComp :type Primitive%20Component%20Object%20Reference) (OtherBodyIndex :type Integer) (bFromSweep :type Boolean) (SweepResult :type Hit%20Result%20Structure%20%28by%20ref%29))
  (Utilities|Casting|CastToBP_MainCharacter OtherActor)
  (bind _returnvalue (UserInterface|CreateWidget "/Game/UI/BP_WGT_Interact.BP_WGT_Interact_C"))
  (UserInterface|Viewport|AddtoViewport _returnvalue 0))

(event OnComponentEndOverlap(Box)
  (params (OverlappedComponent :type Primitive%20Component%20Object%20Reference) (OtherActor :type Actor%20Object%20Reference) (OtherComp :type Primitive%20Component%20Object%20Reference) (OtherBodyIndex :type Integer))
  (Utilities|Casting|CastToBP_MainCharacter OtherActor)
  (Widget|RemovefromParent (stale OnComponentBeginOverlap(Box) _returnvalue)))

(event EventInteract
  (params (FromEnigma? :type Boolean))
  (Class|BPiPlayer|AddMatches(Message) (Game|GetPlayerCharacter 0))
  (Audio|SpawnSoundatLocation "/Game/Sounds/Cues/A_GettingMatches_Cue.A_GettingMatches_Cue" (Transformation|GetWorldLocation (Variables|Default|GetDefaultSceneRoot)) "0, 0, 0" 3.0 1.0 0.0 "/Game/Sounds/Attenuations/Footstep.Footstep" 0)
  (Audio|SpawnSound2D "/Game/Sounds/SFX/Enigmas/Engma_Success01.Engma_Success01" 1.0 1.0 0.0 0)
  (bind _asbp_main_character (Utilities|Casting|CastToBP_MainCharacter (Game|GetPlayerCharacter 0)))
  (Default|ResetMovement _asbp_main_character)
  (Actor|DestroyActor))

(fn ConstructionScript)