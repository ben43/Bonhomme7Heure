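; BP_Timer is a triggerable countdown device that shifts its mesh while running and ticks audibly.
; Trigger, gated by a DoOnce, starts a looping timer calling a custom Tick function that counts up to CountLimit.
; At the limit, TurnTimerOff pauses the timer, restores the mesh, plays a metal-plate sound and re-arms the trigger.
; Interact only resets player movement; range checks and the CursedWood symbol spawn reward are disconnected.
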(event OnComponentBeginOverlap(Box)
  (params (OverlappedComponent :type Primitive%20Component%20Object%20Reference) (OtherActor :type Actor%20Object%20Reference) (OtherComp :type Primitive%20Component%20Object%20Reference) (OtherBodyIndex :type Integer) (bFromSweep :type Boolean) (SweepResult :type Hit%20Result%20Structure%20%28by%20ref%29)))

(event OnComponentEndOverlap(Box)
  (params (OverlappedComponent :type Primitive%20Component%20Object%20Reference) (OtherActor :type Actor%20Object%20Reference) (OtherComp :type Primitive%20Component%20Object%20Reference) (OtherBodyIndex :type Integer)))

(event Custom|TurnTimerOff
  ;[1 1 1] Timer
  (Utilities|Time|PauseTimerbyHandle (stale EventTrigger _returnvalue))
  (CallFunction|ResetTimer)
  (Transformation|AddRelativeLocation (Variables|Default|GetStaticMesh) (* (Variables|Default|GetMeshLocationAdd) "-1.000000,-1.000000,-1.000000") false false)
  (Audio|PlaySoundatLocation "/Game/Sounds/Cues/A_MetalPlate_Cue.A_MetalPlate_Cue" (Transformation|GetActorLocation) "0, 0, 0" 1.0 1.0 0.0 0 0 0))

(event Custom|ResetTimer
  ;[1 1 1] Timer
  (Utilities|FlowControl|DoOnce false) ; enters at Reset
)

(event EventInteract
  (params (FromEnigma? :type Boolean))
  (bind _asbp_main_character (Utilities|Casting|CastToBP_MainCharacter (Game|GetPlayerCharacter 0)))
  (Default|ResetMovement _asbp_main_character))

(event EventBeginPlay)

(event EventTrigger
  (params (Reference :type Actor%20Object%20Reference))
  ;[1 1 1] Timer
  (Utilities|FlowControl|DoOnce false
    (:Completed
      (Transformation|AddRelativeLocation (Variables|Default|GetStaticMesh) (Variables|Default|GetMeshLocationAdd) false false)
      (bind _returnvalue (Utilities|Time|SetTimerbyFunctionName 0 "Tick" 0.2 true))
      (Variables|Default|SetTimer _returnvalue))))

(fn ConstructionScript)

(fn Tick
  (bind _output_get (Variables|Default|SetCounter (+ (Variables|Default|GetCounter) 1)))
  (if (>= _output_get (Variables|Default|GetCountLimit))
    (CallFunction|TurnTimerOff)
    (Variables|Default|SetCounter 0)
    (else
      (Audio|SpawnSoundatLocation "/Game/Sounds/SFX/Clock/ClockTicking-02.ClockTicking-02" (Transformation|GetWorldLocation (Variables|Default|GetStaticMesh)) "0, 0, 0" 1.0 1.0 0.0 "/Game/Sounds/Attenuations/MetalPlate.MetalPlate" 0))))

(fn GetTimerMeshLocation
  (params (Mesh :type Scene%20Component%20Object%20Reference))
  (bind _returnvalue (Transformation|GetWorldLocation Mesh))
  (bind (_x _y _z) (Math|Vector|BreakVector _returnvalue))
  (return (Math|Vector|MakeVector _x _y (+ _z 1e+02))))

(fn SpawnObject
  (params (TimerMeshInput :type Static%20Mesh%20Component%20Object%20Reference))
  (bind _returnvalue (CallFunction|GetTimerMeshLocation TimerMeshInput))
  (Variables|Default|SetTimerMeshLocation _returnvalue)
  (bind _returnvalue_2 (Game|SpawnActorfromClass "/Game/Blueprints/EnigmaBP/BP_SimulatedActor.BP_SimulatedActor_C" (Math|Transform|MakeTransform _returnvalue "0, 0, 0" "1,1,1") "Undefined" 0 0))
  (Components|StaticMesh|SetStaticMesh (Variables|/Game/Blueprints/EnigmaBP/BP_SimulatedActor.BP_SimulatedActor_C|GetStaticMesh _returnvalue_2) "/Game/Models/Props/SM_Symbol_01.SM_Symbol_01")
  (Variables|/Script/Engine.ActorComponent|SetComponentTags (Variables|/Game/Blueprints/EnigmaBP/BP_SimulatedActor.BP_SimulatedActor_C|GetStaticMesh _returnvalue_2) (Utilities|Array|MakeArray "CursedWood"))
  (return))