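; Progression manager that tracks solved enigmas and ends the game when all are finished.
; EnigmaFinishedTrigger increments the finished count and calls CallFinishGame once it reaches TotalNumberOfEnigma.
; A separate UnlockDoors event unlocks the first door after at least one enigma is finished; nothing here calls it.
; The tag-based count of Enigma actors is disconnected, so the total is never computed here, and BeginPlay only runs a delay.
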(event Custom|UnlockDoors
  (if (>= (Variables|Default|GetEnigmaFinished) 1)
    (Variables|/Game/Blueprints/Doors/BP_Door.BP_Door_C|SetLocked? (Variables|Default|Get1stDoorToUnlock) false)))

(event EventBeginPlay
  (Utilities|FlowControl|Delay 0.2))

(event Collision|EventActorBeginOverlap
  (params (OtherActor :type Actor%20Object%20Reference)))

(event EventTick
  (params (DeltaSeconds :type Float%20%28single-precision%29)))

(fn ConstructionScript)

(fn EnigmaFinishedTrigger
  (bind _enigmafinished (Variables|Default|GetEnigmaFinished))
  (Math|Integer|IncrementInt _enigmafinished
    (:%20%20
      (if (>= _enigmafinished (Variables|Default|GetTotalNumberOfEnigma))
        (Default|CallFinishGame)))))