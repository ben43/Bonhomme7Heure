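; Box trigger actor that sends a delayed TriggerMessage to a referenced target when overlapped.
; A DoOnce fires on the first overlap by any actor, then continues only if that actor implements BPi_Interact.
; After the delay, it passes itself to Ref; spawner trigger and 2D sound nodes are left unconnected.
; The construction script sizes the box from BoxExtent.
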(event Collision|EventActorBeginOverlap
  (params (OtherActor :type Actor%20Object%20Reference))
  (Utilities|FlowControl|DoOnce false
    (:Completed
      (if (Utilities|DoesObjectImplementInterface OtherActor "/Game/Blueprints/BPi_Interact.BPi_Interact_C")
        (Utilities|FlowControl|Delay (Variables|Default|GetDelay))
        (Class|BPiInteract|Trigger(Message) (Variables|Default|GetRef) self)))))

(fn ConstructionScript
  (Components|Box|SetBoxExtent (Variables|Default|GetBox) (Variables|Default|GetBoxExtent) true))