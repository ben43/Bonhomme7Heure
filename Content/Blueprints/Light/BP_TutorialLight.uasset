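; BP_TutorialLight is a tutorial light trigger that guides the main character with on-screen text and light beams.
; Entering StartBox shows a tutorial UI widget, then after a delay fades in SecondLightBeam and plays an audio cue.
; A DoOnce blocks retriggering until that timed sequence finishes.
; Leaving EndBox fades out LightBeam, then destroys the associated fill lights and the actor itself.
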(event OnComponentBeginOverlap(StartBox)
  (params (OverlappedComponent :type Primitive%20Component%20Object%20Reference) (OtherActor :type Actor%20Object%20Reference) (OtherComp :type Primitive%20Component%20Object%20Reference) (OtherBodyIndex :type Integer) (bFromSweep :type Boolean) (SweepResult :type Hit%20Result%20Structure%20%28by%20ref%29))
  (Utilities|Casting|CastToBP_MainCharacter OtherActor)
  (Utilities|FlowControl|DoOnce false
    (:Completed
      ;[1 1 1] Display text
      (bind _returnvalue (UserInterface|CreateWidget "/Game/UI/BP_WGT_TutorialUI.BP_WGT_TutorialUI_C"))
      (Variables|/Game/UI/BP_WGT_TutorialUI.BP_WGT_TutorialUI_C|SetTextToSet _returnvalue (Variables|Default|GetText))
      (UserInterface|Viewport|AddtoViewport _returnvalue 0)
      (Utilities|FlowControl|Delay 7.0)
      ;[1 1 1] Fades in next lightbeam
      (Default|Fadein (Variables|Default|GetSecondLightBeam))
      (Audio|SpawnSoundatLocation (Variables|Default|GetSound) (Variables|Default|GetSoundLoc) "0, 0, 0" 1.0 0.7 0.0 0 0) ; Add audio cue
      (Utilities|FlowControl|Delay 5.0)
      (CallFunction|Reset))))

(event OnComponentEndOverlap(EndBox)
  (params (OverlappedComponent :type Primitive%20Component%20Object%20Reference) (OtherActor :type Actor%20Object%20Reference) (OtherComp :type Primitive%20Component%20Object%20Reference) (OtherBodyIndex :type Integer))
  (Utilities|Casting|CastToBP_MainCharacter OtherActor)
  ;[1 1 1] Fades out lightbeam
  (Utilities|FlowControl|Delay 1.0)
  (Default|FadeOut (Variables|Default|GetLightBeam))
  ;[1 1 1] Destroys all fill lights
  (Utilities|FlowControl|Delay 5.0)
  (for _array_element (Variables|Default|GetFillLights)
    (Actor|DestroyActor _array_element))
  (Actor|DestroyActor))

(event Custom|Reset
  (Utilities|FlowControl|DoOnce false) ; enters at Reset
)

(event EventBeginPlay
  (Variables|Default|SetLightBeam (Variables|Default|GetLightBeam)))

(event Collision|EventActorBeginOverlap
  (params (OtherActor :type Actor%20Object%20Reference)))

(event EventTick
  (params (DeltaSeconds :type Float%20%28single-precision%29)))

(fn ConstructionScript)