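; BP_Lights is a configurable spot light that can be switched on and off for night lighting.
; The construction script applies exposed intensity, color, attenuation, cone angle and shadow settings to the SpotLight in candelas.
; BeginPlay caches that intensity as the night value and turns the light off.
; SetNightLights uses a FlipFlop to alternate between restoring the cached intensity and zero on each call.
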(event EventBeginPlay
  (bind _spotlight (Variables|Default|GetSpotLight))
  (Variables|Default|SetNightItensity (Variables|/Script/Engine.LightComponentBase|GetIntensity _spotlight))
  (Rendering|Components|Light|SetIntensity _spotlight 0.0))

(event EventSetNightLights
  (params (Intensity :type Float%20%28single-precision%29))
  (bind _spotlight (Variables|Default|GetSpotLight))
  (Utilities|FlowControl|FlipFlop
    (:A
      (Rendering|Components|Light|SetIntensity _spotlight (Variables|Default|GetNightItensity)))
    (:B
      (Rendering|Components|Light|SetIntensity _spotlight 0.0))))

(fn ConstructionScript
  (bind _spotlight (Variables|Default|GetSpotLight))
  (Class|LocalLightComponent|SetIntensityUnits _spotlight "Candelas")
  (Rendering|Components|Light|SetIntensity _spotlight (Variables|Default|GetIntensity))
  (Rendering|Components|Light|SetLightColor _spotlight (Variables|Default|GetColor) true)
  (Rendering|Lighting|SetAttenuationRadius _spotlight (Variables|Default|GetAttenuation))
  (Rendering|Lighting|SetOuterConeAngle _spotlight (Variables|Default|GetOuterConeAngle))
  (Rendering|Components|Light|SetCastShadows _spotlight (Variables|Default|GetCastShadow)))