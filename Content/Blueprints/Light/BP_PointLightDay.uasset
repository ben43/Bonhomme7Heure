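; BP_PointLightDay is a point light that shines by day and turns off at night.
; On BeginPlay it caches the PointLight component's intensity, unless ManualIntensity keeps the Intensity variable as set, then zeroes the light.
; SetDayLights restores the stored intensity and SetNightLights sets it to zero, with neither event called within this Blueprint.
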(event EventBeginPlay
  (if (Variables|Optional|GetManualIntensity)
    _
    (else
      (Variables|Optional|SetIntensity (Variables|/Script/Engine.LightComponentBase|GetIntensity (Variables|Default|GetPointLight)))))
  (Rendering|Components|Light|SetIntensity (Variables|Default|GetPointLight) 0.0))

(event EventSetDayLights
  (params (Intensity :type Float%20%28single-precision%29))
  (Rendering|Components|Light|SetIntensity (Variables|Default|GetPointLight) (Variables|Optional|GetIntensity)))

(event EventSetNightLights
  (params (Intensity :type Float%20%28single-precision%29))
  (Rendering|Components|Light|SetIntensity (Variables|Default|GetPointLight) 0.0))

(fn ConstructionScript)