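; BP_Key is an interactable key actor that unlocks the door it references.
; On Interact, it casts the player character to BP_MainCharacter, resets its movement and clears the Locked flag on DoorReference.
; It then plays a 2D success sound, spawns a particle effect at the key's mesh location and destroys itself.
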(event EventBeginPlay)

(event Collision|EventActorBeginOverlap
  (params (OtherActor :type Actor%20Object%20Reference)))

(event EventTick
  (params (DeltaSeconds :type Float%20%28single-precision%29)))

(event EventInteract
  (params (FromEnigma? :type Boolean))
  (bind _asbp_main_character (Utilities|Casting|CastToBP_MainCharacter (Game|GetPlayerCharacter 0)))
  (Default|ResetMovement _asbp_main_character)
  (Variables|/Game/Blueprints/Doors/BP_Door.BP_Door_C|SetLocked? (Variables|Default|GetDoorReference) false)
  (Audio|SpawnSound2D "/Game/Sounds/SFX/Enigmas/Engma_Success01.Engma_Success01" 1.0 1.0 0.0 0)
  (Effects|SpawnEmitteratLocation (Variables|Default|GetParticlesSpawn) (Transformation|GetWorldLocation (Variables|Default|GetStaticMesh)))
  (Actor|DestroyActor))

(fn ConstructionScript)