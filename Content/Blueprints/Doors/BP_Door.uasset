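; Physics-driven door that adult characters open and close, with locked and unlocked sounds.
; A box overlap shows the interact widget to adult and child characters, but only adults can operate it; FromEnigma calls bypass range and lock checks.
; Interact flip-flops physics constraint velocity and an impulse, disabling simulation after closing.
; A separate AI collision lets BP_AI_7OCLOCK snap it 90 degrees open and back unless OpenedByPlayer is set.
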(event OnComponentBeginOverlap(Box)
  (params (OverlappedComponent :type Primitive%20Component%20Object%20Reference) (OtherActor :type Actor%20Object%20Reference) (OtherComp :type Primitive%20Component%20Object%20Reference) (OtherBodyIndex :type Integer) (bFromSweep :type Boolean) (SweepResult :type Hit%20Result%20Structure%20%28by%20ref%29))
  (Utilities|Casting|CastToBP_AdultCharacter OtherActor
    (:then
      (bind _returnvalue (UserInterface|CreateWidget "/Game/UI/BP_WGT_Interact.BP_WGT_Interact_C"))
      (bind _output_get (Variables|Default|SetInteractWidget _returnvalue))
      (UserInterface|Viewport|AddtoViewport _output_get 0)
      (Variables|Default|SetCharacterInRange true)
      (Variables|Default|SetAdultCharacter? true))
    (:CastFailed
      (Utilities|Casting|CastToBP_ChildCharacter OtherActor)
      (bind _returnvalue_2 (UserInterface|CreateWidget "/Game/UI/BP_WGT_Interact.BP_WGT_Interact_C"))
      (bind _output_get_2 (Variables|Default|SetInteractWidget _returnvalue_2))
      (UserInterface|Viewport|AddtoViewport _output_get_2 0)
      (Variables|Default|SetAdultCharacter? false)
      (Variables|Default|SetCharacterInRange true))))

(event OnComponentEndOverlap(Box)
  (params (OverlappedComponent :type Primitive%20Component%20Object%20Reference) (OtherActor :type Actor%20Object%20Reference) (OtherComp :type Primitive%20Component%20Object%20Reference) (OtherBodyIndex :type Integer))
  (bind _interactwidget (Variables|Default|GetInteractWidget))
  (Utilities|Casting|CastToBP_AdultCharacter OtherActor
    (:then
      (Widget|RemovefromParent _interactwidget)
      (Variables|Default|SetCharacterInRange false))
    (:CastFailed
      (Utilities|Casting|CastToBP_ChildCharacter OtherActor)
      (Widget|RemovefromParent _interactwidget)
      (Variables|Default|SetCharacterInRange false))))

(event OnComponentBeginOverlap(AICollision)
  (params (OverlappedComponent :type Primitive%20Component%20Object%20Reference) (OtherActor :type Actor%20Object%20Reference) (OtherComp :type Primitive%20Component%20Object%20Reference) (OtherBodyIndex :type Integer) (bFromSweep :type Boolean) (SweepResult :type Hit%20Result%20Structure%20%28by%20ref%29))
  (Utilities|Casting|CastToBP_AI_7OCLOCK OtherActor)
  (CallFunction|OpenDoor))

(event OnComponentEndOverlap(AICollision)
  (params (OverlappedComponent :type Primitive%20Component%20Object%20Reference) (OtherActor :type Actor%20Object%20Reference) (OtherComp :type Primitive%20Component%20Object%20Reference) (OtherBodyIndex :type Integer))
  (Utilities|Casting|CastToBP_AI_7OCLOCK OtherActor)
  (CallFunction|CloseDoor))

(event Custom|OpenDoor
  (bind _doormesh (Variables|Default|GetDoorMesh))
  (bind _returnvalue (Transformation|GetWorldRotation _doormesh))
  (bind (_roll _pitch _yaw) (Math|Rotator|BreakRotator _returnvalue))
  (if (not (Variables|Default|GetOpenedByPlayer))
    (Utilities|FlowControl|DoOnce false
      (:Completed
        (Transformation|SetWorldRotation _doormesh (Math|Rotator|MakeRotator _roll _pitch (+ _yaw 9e+01)) false false)
        (Utilities|FlowControl|DoOnce false) ; enters at Reset
      ))))

(event Custom|Close%20Door
  (bind _doormesh (Variables|Default|GetDoorMesh))
  (bind _returnvalue (Transformation|GetWorldRotation _doormesh))
  (bind (_roll _pitch _yaw) (Math|Rotator|BreakRotator _returnvalue))
  (if (not (Variables|Default|GetOpenedByPlayer))
    (Utilities|FlowControl|DoOnce false
      (:Completed
        (Transformation|SetWorldRotation _doormesh (Math|Rotator|MakeRotator _roll _pitch (- _yaw 9e+01)) false false)
        (Utilities|FlowControl|DoOnce false) ; enters at Reset
      ))))

(event EventInteract
  (params (FromEnigma? :type Boolean))
  (bind _audio (Variables|Default|GetAudio))
  (bind _asbp_main_character (Utilities|Casting|CastToBP_MainCharacter (Game|GetPlayerCharacter 0)))
  (Default|ResetMovement _asbp_main_character)
  (if FromEnigma?
    (Utilities|FlowControl|FlipFlop :!label _label
      (:A
        ;[1 1 1] Door open
        (if (Variables|Default|GetWasLocked)
          (Audio|SpawnSoundatLocation "/Game/Sounds/SFX/Door/DoorUnlocked.DoorUnlocked" (Transformation|GetActorLocation (Game|GetPlayerCharacter 0)) "0, 0, 0" 1.0 1.0 0.0 "/Game/Sounds/Attenuations/Footstep.Footstep" 0))
        (Physics|SetSimulatePhysics (Variables|Default|GetDoorMesh) true)
        (Class|PhysicsConstraintComponent|SetAngularVelocityTarget (Variables|Default|GetPhysicsConstraint) (Math|Vector|MakeVector 0.0 0.0 -0.05))
        ;[1 1 1] Audio
        (Audio|Components|Audio|SetSound _audio (Variables|Default|GetDoopOpen))
        (Audio|Components|Audio|Play _audio 0.0)
        (Variables|Default|SetOpenedByPlayer true))
      (:B
        ;[1 1 1] Door close
        (Physics|AddImpulse (Variables|Default|GetDoorMesh) "0,1000.000000, 0" "None" false)
        (Class|PhysicsConstraintComponent|SetAngularVelocityTarget (Variables|Default|GetPhysicsConstraint) (Variables|Default|GetVelocityTarget))
        (Utilities|FlowControl|Sequence
          (:then_0
            (Audio|Components|Audio|SetSound _audio (Variables|Default|GetDoorClose))
            (Audio|Components|Audio|Play _audio 0.0)
            (Variables|Default|SetOpenedByPlayer false))
          (:then_1
            ;[1 1 1] Turn Simulation Off when Closed
            (Utilities|FlowControl|Delay 2.0)
            (Physics|SetSimulatePhysics (Variables|Default|GetDoorMesh) false)))))
    (elif (Variables|Default|GetLocked?)
      ;[1 1 1] Locked Audio
      (Audio|SpawnSoundatLocation "/Game/Sounds/Cues/A_DoorLocked_Cue.A_DoorLocked_Cue" (Transformation|GetActorLocation (Game|GetPlayerCharacter 0)) "0, 0, 0" 3.0 1.0 0.0 "/Game/Sounds/Attenuations/Footstep.Footstep" 0)
      (Variables|Default|SetWasLocked true)
      (elif (Variables|Default|GetCharacterInRange)
        (if (Variables|Default|GetAdultCharacter?)
          (goto _label))))))

(fn ConstructionScript)