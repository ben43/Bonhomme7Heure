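; Door trap actor that reacts to an overlap by jumping upward with a sound.
; The construction script applies configurable mesh, box scale and audio settings.
; A box overlap sends the Interact message when the other actor implements BPi_Interact.
; Interact sets relative location from the box's world position plus a Z offset, through a single VInterpTo call without delta time or speed, then plays audio.
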(event OnComponentBeginOverlap(Box)
  (params (OverlappedComponent :type Primitive%20Component%20Object%20Reference) (OtherActor :type Actor%20Object%20Reference) (OtherComp :type Primitive%20Component%20Object%20Reference) (OtherBodyIndex :type Integer) (bFromSweep :type Boolean) (SweepResult :type Hit%20Result%20Structure%20%28by%20ref%29))
  (if (Utilities|DoesObjectImplementInterface OtherActor "/Game/Blueprints/BPi_Interact.BPi_Interact_C")
    (Class|BPiInteract|Interact(Message) self)))

(event EventBeginPlay)

(event Collision|EventActorBeginOverlap
  (params (OtherActor :type Actor%20Object%20Reference)))

(event EventTick
  (params (DeltaSeconds :type Float%20%28single-precision%29)))

(fn ConstructionScript
  (bind _audio (Variables|Default|GetAudio))
  (Components|StaticMesh|SetStaticMesh (Variables|Default|GetStaticMesh) (Variables|Default|GetTrap%20Mesh))
  (Transformation|SetRelativeScale3D (Variables|Default|GetBox) (Variables|Default|GetBox%20Scale))
  (Audio|Components|Audio|SetSound _audio (Variables|Default|GetAudioSound))
  (Audio|Components|Audio|SetVolumeMultiplier _audio (Variables|Default|GetAudioVolume) :!class /Script/Engine.AudioComponent))

(fn Interact
  (bind _box (Variables|Default|GetBox))
  (bind _returnvalue (Transformation|GetWorldLocation _box))
  (Transformation|SetActorRelativeLocation (Math|Interpolation|VInterpTo _returnvalue (+ _returnvalue "0, 0,50.000000") 0.0 0.0))
  (Audio|Components|Audio|Play (Variables|Default|GetAudio) 0.0)
  (return))